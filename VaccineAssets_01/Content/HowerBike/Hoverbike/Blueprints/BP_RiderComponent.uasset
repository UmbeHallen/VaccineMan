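; Rider component that lets its owning Character spawn, mount and dismount a BP_HoverBike.
; SpawnBike sphere-traces forward, then top-down if blocked, and teleports and resets the previous unmounted bike instead of spawning another.
; Mount and Dismount swap possession and movement state, with dismount teleporting the rider and briefly ignoring Vehicle collision via a timer.
; ShowArms toggles visibility between the character mesh and an arms mesh.
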(event `self.ReceiveBeginPlay`)

(fn `CharacterBlockVehicles`
  (bind _ascharacter (cast `Character` (`self.GetOwner`)))
  (`PrimitiveComponent.SetCollisionResponseToChannel` (`Character.CapsuleComponent` _ascharacter) "ECC_Vehicle" "ECR_Block"))

(fn `Dismount`
  (params (MountTrigger :type "SceneComponent Object Reference") (DestLocation :type "Vector Structure") (DestRotation :type "Rotator Structure") (CanUnmountFromLeft :type Boolean))
  (returns (`CouldDismount?` :type Boolean))
  (bind _returnvalue (`self.GetOwner`))
  (`/Engine/EditorBlueprintResources/StandardMacros.IsValid` MountTrigger
    (:`Is Valid`
      (bind _ascharacter (cast `Character` _returnvalue)
        (:`then`
          (`self.SetActive` (`Character.CharacterMovement` _ascharacter) true true)
          (set `self.CanUnmountFromLeft` CanUnmountFromLeft)
          (`Actor.K2_TeleportTo` _returnvalue (`local.DestLocation`) (`local.DestRotation`))
          (`Controller.Possess` (`Pawn.GetController` (`self.CurrentHoverBikeRef`)) _ascharacter)
          (`Actor.K2_DetachFromActor` _ascharacter "KeepWorld" "KeepWorld" "KeepWorld")
          (`Actor.SetActorEnableCollision` _ascharacter true)
          (`PrimitiveComponent.SetCollisionResponseToChannel` (`Character.CapsuleComponent` _ascharacter) "ECC_Vehicle" "ECR_Ignore")
          (`KismetSystemLibrary.K2_SetTimer` null "CharacterBlockVehicles" 0.5)
          (set `self.IsRidingBike` false)
          (return true))
        (:`CastFailed`
          (`KismetSystemLibrary.PrintString` "MESSAGE: Not a Rider")
          (return false))))
    (:`Is Not Valid`
      (return false))))

(fn `Mount`
  (bind _currenthoverbikeref (`self.CurrentHoverBikeRef`))
  (bind _currenthoverbikeref_2 (`self.CurrentHoverBikeRef`))
  (`/Engine/EditorBlueprintResources/StandardMacros.IsValid` _currenthoverbikeref_2
    (:`Is Valid`
      (if (and (`self.CanMount`) (not (`/Game/HowerBike/Hoverbike/Blueprints/BP_HoverBike.IsCurrentlyMounted` _currenthoverbikeref_2)))
        (bind _ascharacter (cast `Character` (`self.GetOwner`))
          (:`then`
            (bind _charactermovement (`Character.CharacterMovement` _ascharacter))
            (`MovementComponent.StopMovementImmediately` _charactermovement)
            (`self.Deactivate` _charactermovement)
            (`Controller.Possess` (`Pawn.GetController` _ascharacter) _currenthoverbikeref)
            (`/Game/HowerBike/Hoverbike/Blueprints/BP_HoverBike.MountBike` _currenthoverbikeref _ascharacter)
            (set `self.IsRidingBike` true))
          (:`CastFailed`
            (`KismetSystemLibrary.PrintString` "Not a Rider character")))))))

(fn `ShowArms`
  (params (`ShowArms?` :type Boolean))
  (bind _armsmesh (`self.ArmsMesh`))
  (bind _ascharacter (cast `Character` (`self.GetOwner`)))
  (bind _mesh (`Character.Mesh` _ascharacter))
  (`SceneComponent.SetHiddenInGame` _mesh `ShowArms?` false)
  (`SceneComponent.SetVisibility` _mesh (not `ShowArms?`) false)
  (`/Engine/EditorBlueprintResources/StandardMacros.IsValid` _armsmesh
    (:`Is Valid`
      (`SceneComponent.SetHiddenInGame` _armsmesh (not `ShowArms?`) false)
      (`SceneComponent.SetVisibility` _armsmesh `ShowArms?` false))))

(fn `SpawnBike`
  (locals (SpawningRot :type "Rotator Structure" :default (struct)) (SpawningScale :type "Vector Structure" :default (0.0 0.0 0.0)) (SpawningLocation :type "Vector Structure"))
  (bind _returnvalue (`self.GetOwner`))
  (bind _returnvalue_2 (`self.GetOwner`))
  (bind _spawnedhoverbikeref (`self.SpawnedHoverBikeRef`))
  (bind (_returnvalue_location _returnvalue_rotation _returnvalue_scale) (`KismetMathLibrary.BreakTransform` (`Actor.GetTransform` _returnvalue)))
  ;[1 1 1] Check if there is something in front of us that can block the hoverbike spawn
  (set `local.SpawningRot` (`KismetMathLibrary.Conv_VectorToRotator` (`Actor.GetActorRightVector` _returnvalue)))
  (set `local.SpawningScale` _returnvalue_scale)
  (set `local.SpawningLocation` (+ _returnvalue_location (* (`Actor.GetActorForwardVector` _returnvalue) 300.0) (0.0 0.0 40.0)))
  (bind (_outhit _returnvalue_3) (`KismetSystemLibrary.SphereTraceSingleForObjects` _returnvalue_location (`local.SpawningLocation`) 50.0 (`|MakeArray` "ObjectTypeQuery1" "ObjectTypeQuery2" "ObjectTypeQuery3" :!type "EObjectTypeQuery Enum"))) ; Try frontal approach
  (if _returnvalue_3
    (bind (_bblockinghit _binitialoverlap _time _distance _location _impactpoint _normal _impactnormal _physmat _hitactor _hitcomponent _hitbonename _hititem _elementindex _faceindex _tracestart _traceend) (`GameplayStatics.BreakHitResult` _outhit))
    ;[1 1 1] Collision check from top to bottom to see if we can still spawn the hoverbike
    (bind (_outhit_2 _returnvalue_4) (`KismetSystemLibrary.SphereTraceSingleForObjects` (+ _traceend (0.0 0.0 100.0)) _traceend 70.0 (`|MakeArray` "ObjectTypeQuery1" "ObjectTypeQuery2" "ObjectTypeQuery3" :!type "EObjectTypeQuery Enum"))) ; Try top down approach
    (if _returnvalue_4
      (bind (_bblockinghit_2 _binitialoverlap_2 _time_2 _distance_2 _location_2 _impactpoint_2 _normal_2 _impactnormal_2 _physmat_2 _hitactor_2 _hitcomponent_2 _hitbonename_2 _hititem_2 _elementindex_2 _faceindex_2 _tracestart_2 _traceend_2) (`GameplayStatics.BreakHitResult` _outhit_2))
      (if (< (`KismetMathLibrary.VSize` (- _traceend _impactpoint_2)) 90.0)
        (set `local.SpawningLocation` (+ (`KismetMathLibrary.SelectVector` _impactpoint_2 _traceend_2 _returnvalue_4) (0.0 0.0 100.0)) :!label _label)
        ;[1 1 1] lets spawn the hoverbike if we haven't done it before or if the bike is being used by someone else, otherwise teleport the old hoverbike and reset its values to give the ilusion of spawning a new one without having to destroy and create it again (spawning actors is expensive)
        (`/Engine/EditorBlueprintResources/StandardMacros.IsValid` _spawnedhoverbikeref :!label _label_2
          (:`Is Valid`
            (if (not (`/Game/HowerBike/Hoverbike/Blueprints/BP_HoverBike.IsCurrentlyMounted` _spawnedhoverbikeref))
              (`Actor.K2_SetActorLocationAndRotation` _spawnedhoverbikeref (`local.SpawningLocation`) (`local.SpawningRot`) false true)
              (`/Game/HowerBike/Hoverbike/Blueprints/BP_HoverBike.ServerReset` _spawnedhoverbikeref)
              (else
                (bind _returnvalue_5 (`|SpawnActorFromClass` "/Game/HowerBike/Hoverbike/Blueprints/BP_HoverBike.BP_HoverBike_C" (`KismetMathLibrary.MakeTransform` (`local.SpawningLocation`) (`local.SpawningRot`) (`local.SpawningScale`)) "AdjustIfPossibleButAlwaysSpawn" "OverrideRootScale" _returnvalue_2 (cast `Pawn` _returnvalue_2 :!pure true) :!label _label_3))
                (bind _output_get (set `self.SpawnedHoverBikeRef` _returnvalue_5))
                (`Pawn.SpawnDefaultController` _output_get))))
          (:`Is Not Valid`
            (goto _label_3)))
        (else
          ;[1 1 1] Debug message informing that there is not a valid location to spawn a hoverbike
          (`KismetSystemLibrary.PrintString` "BP_RiderComponent (SpawnBike function): No valid location in front of player)")))
      (else
        (goto _label)))
    (else
      (goto _label_2))))