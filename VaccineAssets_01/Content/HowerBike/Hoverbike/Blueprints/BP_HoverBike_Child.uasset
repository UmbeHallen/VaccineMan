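; Hoverbike child Blueprint that adds player camera look, free turret rotation and shooting.
; Turn and LookUp axes feed the camera controller, while holding right mouse toggles free camera rotation on the turret controller.
; Left mouse plays a timeline that spawns a player projectile at the emitter's transform on every update until release or timeline end.
; Gun-mode MultiGate and shooting VFX nodes are present but unconnected.
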(event `Key|RightMouseButton`
  (params (Key :type "Key Structure"))
  (:`Pressed`
    (set `self.Free Rotation` true)
    (`/Game/ASSETS/CODE/Turret_Controller/Blueprints/Turret_controller_BP.Free Camera Rotation` (`self.Turret_controller_BP`) (stale _output_get) :!label _label))
  (:`Released`
    (bind _output_get (set `self.Free Rotation` false))
    (goto _label)))

(event `InputAxis|Turn`
  (params (AxisValue :type "Float (single-precision)"))
  (`/Game/ASSETS/CODE/Turret_Controller/Blueprints/Camera_Controller_BP.Add look at direction (Camera)` (`self.Camera_Controller_BP`) AxisValue (stale `InputAxis|LookUp` AxisValue) :!label _label_2))

(event `InputAxis|LookUp`
  (params (AxisValue :type "Float (single-precision)"))
  (goto _label_2))

(event `Key|LeftMouseButton`
  (params (Key :type "Key Structure"))
  (bind (_returnvalue_location _returnvalue_rotation) (`KismetMathLibrary.BreakTransform` (`SceneComponent.K2_GetComponentToWorld` (`self.Emitter1`))))
  ;[0 0 0] FireLogic
  (:`Pressed`
    (`Timeline|Timeline_1` :!via `PlayFromStart` :!label _label_3
      (:`Update`
        (`|SpawnActorFromClass` "/Game/GAME_FOLDER/CORE/BLUEPRINTS/PROJECTILES/BP_PlayerProjectileBase1.BP_PlayerProjectileBase1_C" (`KismetMathLibrary.MakeTransform` _returnvalue_location _returnvalue_rotation (1.0 1.0 1.0)) "AdjustIfPossibleButAlwaysSpawn" "OverrideRootScale" self self))))
  (:`Released`
    (goto _label_3 :!via `Stop`)))

(fn `UserConstructionScript`
  (`parent.UserConstructionScript`))