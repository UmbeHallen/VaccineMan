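; Blood-themed shield effect actor that reacts visually wherever its sphere mesh is hit.
; Each hit passes the impact point to the shield Niagara system and a new dynamic blood material, then spawns a blood burst along the impact normal.
; A restarted timeline animates the Niagara hit radius and the material's vertex noise and hit opacity, while the material's hit radius is multiplied to zero.
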(event `self.ReceiveBeginPlay`
  (`self.EnableInput` (`GameplayStatics.GetPlayerController` 0)))

(event `self.SM_Sphere.OnComponentHit`
  (params (HitComponent :type "PrimitiveComponent Object Reference") (OtherActor :type "Actor Object Reference") (OtherComp :type "PrimitiveComponent Object Reference") (NormalImpulse :type "Vector Structure") (Hit :type "HitResult Structure (by ref)"))
  ;[1 1 1] Niagara
  (`NiagaraComponent.SetVariableVec3` (`self.NS_Shield_Sphere`) "Hit_SphereLocation" Hit_ImpactPoint)
  ;[1 1 1] Mesh
  (bind _returnvalue (`PrimitiveComponent.CreateDynamicMaterialInstance` (`self.SM_Sphere`) 0 "/Game/ASSETS/VFX/Shield_FX_Niagara/Niagara_Shield/Material/M_Shield_Blood.M_Shield_Blood" "None"))
  (`MaterialInstanceDynamic.SetVectorParameterValue` _returnvalue "Hit_Location" (`KismetMathLibrary.Conv_VectorToLinearColor` Hit_ImpactPoint))
  (`NiagaraFunctionLibrary.SpawnSystemAtLocation` "/Game/ASSETS/VFX/Shield_FX_Niagara/Hit_Particles/NS_Hit_Blood.NS_Hit_Blood" Hit_ImpactPoint (`KismetMathLibrary.MakeRotFromZ` Hit_ImpactNormal))
  (bind (_direction _vertexnoise_strength _hit_opacity _radius_hit _vertexnoise_radius _niagara_hit_radius) (`Timeline|Mesh_Timeline` :!via `PlayFromStart`)
    (:`Update`
      (`NiagaraComponent.SetVariableFloat` (`self.NS_Shield_Sphere`) "Hit_SphereRadius" (* _niagara_hit_radius (`self.Niagara_Hit_Radius`)))
      (`MaterialInstanceDynamic.SetScalarParameterValue` _returnvalue "Radius_VertexNoise" (* _vertexnoise_radius (`self.Radius_VertexNoise`)))
      (`MaterialInstanceDynamic.SetScalarParameterValue` _returnvalue "Strength_VertexNoise" (* _vertexnoise_strength (`self.VertexNoise_Strength`)))
      (`MaterialInstanceDynamic.SetScalarParameterValue` _returnvalue "Hit_opacity" _hit_opacity)
      (`MaterialInstanceDynamic.SetScalarParameterValue` _returnvalue "radius_Hit" (* _radius_hit (`self.radius_Hit`) 0.0)))))

(fn `UserConstructionScript`)