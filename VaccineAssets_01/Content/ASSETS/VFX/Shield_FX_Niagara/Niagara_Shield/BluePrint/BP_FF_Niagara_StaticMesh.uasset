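; Niagara shield actor on a static mesh sphere that shows an impact reaction wherever something hits it.
; On component hit, it passes the impact point to the shield's Niagara system and a newly created dynamic material on the mesh.
; It also spawns a gold hit effect oriented along the impact normal.
; A timeline then drives the Niagara hit radius, scaled by a radius variable.
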(event `self.ReceiveBeginPlay`
  (`self.EnableInput` (`GameplayStatics.GetPlayerController` 0)))

(event `self.SM_Sphere.OnComponentHit`
  (params (HitComponent :type "PrimitiveComponent Object Reference") (OtherActor :type "Actor Object Reference") (OtherComp :type "PrimitiveComponent Object Reference") (NormalImpulse :type "Vector Structure") (Hit :type "HitResult Structure (by ref)"))
  ;[1 1 1] Niagara
  (`NiagaraComponent.SetVariableVec3` (`self.NS_Shield_Sprite_GeoSphere_01`) "Hit_SphereLocation" Hit_ImpactPoint)
  ;[1 1 1] Mesh
  (bind _returnvalue (`PrimitiveComponent.CreateDynamicMaterialInstance` (`self.SM_Sphere`) 0 "/Game/ASSETS/VFX/Shield_FX_Niagara/Niagara_Shield/Material/M_Transparent.M_Transparent" "None"))
  (`MaterialInstanceDynamic.SetVectorParameterValue` _returnvalue "Hit_Location" (`KismetMathLibrary.Conv_VectorToLinearColor` Hit_ImpactPoint))
  (`NiagaraFunctionLibrary.SpawnSystemAtLocation` "/Game/ASSETS/VFX/Shield_FX_Niagara/Hit_Particles/NS_Hit_Gold.NS_Hit_Gold" Hit_ImpactPoint (`KismetMathLibrary.MakeRotFromZ` Hit_ImpactNormal))
  (bind (_direction _niagara_hit_radius) (`Timeline|Mesh_Timeline` :!via `PlayFromStart`)
    (:`Update`
      (`NiagaraComponent.SetVariableFloat` (`self.NS_Shield_Sprite_GeoSphere_01`) "Hit_SphereRadius" (* _niagara_hit_radius (`self.Niagara_Hit_Radius`))))))

(fn `UserConstructionScript`)