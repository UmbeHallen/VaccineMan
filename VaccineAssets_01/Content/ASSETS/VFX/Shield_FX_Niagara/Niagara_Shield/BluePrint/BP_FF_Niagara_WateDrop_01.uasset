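; Water-drop shield pod actor that randomizes its scale and type (A, PA, P, E), spawns a turret and flags when a Main_Interface actor is in range.
; Construction sets core material color and Niagara spawn rates by type.
; Hits spawn a bubble effect and start a timeline animating Niagara hit radius and material vertex noise.
; Each timeline update calls OnTakingDmg, whose MultiGate destroys the actor on its third output.
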(event `self.SM_Sphere.OnComponentHit`
  (params (HitComponent :type "PrimitiveComponent Object Reference") (OtherActor :type "Actor Object Reference") (OtherComp :type "PrimitiveComponent Object Reference") (NormalImpulse :type "Vector Structure") (Hit :type "HitResult Structure (by ref)"))
  ;[1 1 1 1 30] HIT EFFECT
  ;;[1 1 1] Niagara
  (`NiagaraComponent.SetVariableVec3` (`self.NS_Shield_Sphere`) "Hit_SphereLocation" Hit_ImpactPoint)
  ;;[1 1 1] Mesh
  (bind _returnvalue (`PrimitiveComponent.CreateDynamicMaterialInstance` (`self.SM_Sphere`) 0 "/Game/ASSETS/VFX/Shield_FX_Niagara/Niagara_Shield/Material/M_waterDrop.M_waterDrop" "None"))
  (`MaterialInstanceDynamic.SetVectorParameterValue` _returnvalue "Hit_Location" (`KismetMathLibrary.Conv_VectorToLinearColor` Hit_ImpactPoint))
  (`NiagaraFunctionLibrary.SpawnSystemAtLocation` "/Game/ASSETS/VFX/Shield_FX_Niagara/Hit_Particles/NS_Hit_Bubble.NS_Hit_Bubble" Hit_ImpactPoint (`KismetMathLibrary.MakeRotFromZ` Hit_ImpactNormal))
  (bind (_direction _vertexnoise_strength _hit_opacity _radius_hit _vertexnoise_radius _niagara_hit_radius) (`Timeline|Mesh_Timeline` :!via `PlayFromStart`)
    (:`Update`
      (`NiagaraComponent.SetVariableFloat` (`self.NS_Shield_Sphere`) "Hit_SphereRadius" (* _niagara_hit_radius (`self.Niagara_Hit_Radius`)))
      (`MaterialInstanceDynamic.SetScalarParameterValue` _returnvalue "Radius_VertexNoise" (* _vertexnoise_radius (`self.Radius_VertexNoise`)))
      (`MaterialInstanceDynamic.SetScalarParameterValue` _returnvalue "Strength_VertexNoise" (* _vertexnoise_strength (`self.VertexNoise_Strength`)))
      (`MaterialInstanceDynamic.SetScalarParameterValue` _returnvalue "Hit_opacity" _hit_opacity)
      (`MaterialInstanceDynamic.SetScalarParameterValue` _returnvalue "radius_Hit" (* _radius_hit (`self.radius_Hit`) 0.0))
      (`self.OnTakingDmg`))))

(event `self.ReceiveBeginPlay`
  (`self.EnableInput` (`GameplayStatics.GetPlayerController` 0))
  (bind _returnvalue (`|SpawnActorFromClass` "/Game/ASSETS/CODE/UnderSiege/BluePrints/Turret/BP_USTurret3.BP_USTurret3_C" (`KismetMathLibrary.MakeTransform` (`self.K2_GetActorLocation`) (`SceneComponent.K2_GetComponentRotation` (`self.Arrow`))) "AdjustIfPossibleButAlwaysSpawn" "OverrideRootScale" null null))
  (set `self.Turret_ref` _returnvalue))

(event `self.Sphere.OnComponentBeginOverlap`
  (params (OverlappedComponent :type "PrimitiveComponent Object Reference") (OtherActor :type "Actor Object Reference") (OtherComp :type "PrimitiveComponent Object Reference") (OtherBodyIndex :type Integer) (bFromSweep :type Boolean) (SweepResult :type "HitResult Structure (by ref)"))
  ;[0 0 0] TRIGGER
  (if (`KismetSystemLibrary.DoesImplementInterface` OtherActor "/Game/GAME_FOLDER/CORE/UTILITY/Main_Interface.Main_Interface_C")
    (bind _output_get (set `self.PlayerInRange` true))
    (`KismetSystemLibrary.PrintString` (`KismetStringLibrary.Conv_BoolToString` _output_get))))

(event `self.Sphere.OnComponentEndOverlap`
  (params (OverlappedComponent :type "PrimitiveComponent Object Reference") (OtherActor :type "Actor Object Reference") (OtherComp :type "PrimitiveComponent Object Reference") (OtherBodyIndex :type Integer))
  ;[0 0 0] TRIGGER
  (if (`KismetSystemLibrary.DoesImplementInterface` OtherActor "/Game/GAME_FOLDER/CORE/UTILITY/Main_Interface.Main_Interface_C")
    (set `self.PlayerInRange` false)))

(event `OnTakingDmg`
  (`|MultiGate` false
    (:`Out 2`
      (`self.K2_DestroyActor`))))

(fn `GetNiagaraEffect`
  (returns (NS_Shield_Sphere :type "NiagaraComponent Object Reference"))
  (return (`self.NS_Shield_Sphere`)))

(fn `SendTurretInfo`
  (returns (TurretRef :type "Actor Object Reference"))
  (return (`self.Turret_ref`)))

(fn `UserConstructionScript`
  (bind _returnvalue (`KismetMathLibrary.RandomFloatInRange` 1.0 6.0))
  (bind _ns_shield_sphere (`self.NS_Shield_Sphere`))
  (bind _ns_shield_sphere_2 (`self.NS_Shield_Sphere`))
  ;[0 0 0] MaterialInstance SetUp
  (bind _returnvalue_2 (`PrimitiveComponent.CreateDynamicMaterialInstance` (`self.Core`) 0 "/Game/ASSETS/MATERIALS/MaterialFunctionCollection/Materials/Materials/Edge_Fade/M_StatueGlass_EdgeFade_02_Inst.M_StatueGlass_EdgeFade_02_Inst" "None"))
  (set `self.Core_Material` _returnvalue_2)
  (`self.SetActorScale3D` (`KismetMathLibrary.MakeVector` _returnvalue _returnvalue _returnvalue))
  ;[0 0 0] Randomize TYPE
  (bind _output_get (set `self.PodType_Nr` (`KismetMathLibrary.RandomIntegerInRange` 0 10)))
  (switch `int` _output_get
    (:`0`
      (set `self.PodType_ID` "A" :!label _label))
    (:`1`
      (goto _label))
    (:`2`
      (goto _label))
    (:`3`
      (set `self.PodType_ID` "PA" :!label _label_2))
    (:`4`
      (goto _label_2))
    (:`5`
      (goto _label_2))
    (:`6`
      (goto _label_2))
    (:`7`
      (set `self.PodType_ID` "P" :!label _label_3))
    (:`8`
      (goto _label_3))
    (:`9`
      (set `self.PodType_ID` "E")))
  ;[0 0 0] SET UP ACCORDING TO TYPE
  (switch `string` (`self.PodType_ID`)
    (:`A`
      (`|ExecutionSequence`
        (:`then_0`
          ;[0 0 0] AGGRESIVE TYPE MATERIAL COLOR
          (`MaterialInstanceDynamic.SetVectorParameterValue` (`self.Core_Material`) "ColorGlass" (struct :`R` 1.0 :`G` 0.007345 :`A` 1.0)))
        (:`then_1`
          (`MaterialInstanceDynamic.SetVectorParameterValue` (`self.Core_Material`) "F_Color" (struct :`R` 20.0 :`G` 1.059936 :`A` 1.0))
          (`NiagaraComponent.SetVariableFloat` _ns_shield_sphere_2 "SpawnRate01" 5.0)
          (`NiagaraComponent.SetVariableFloat` _ns_shield_sphere_2 "SpawnRate02" 10.0))))
    (:`PA`
      ;[0 0 0] AGGRESIVE TYPE MATERIAL COLOR
      (`MaterialInstanceDynamic.SetVectorParameterValue` (`self.Core_Material`) "ColorGlass" (`KismetMathLibrary.LinearColorLerp` (`self.Color_Picker_A`) (`self.Color_Picker_B`) (`KismetMathLibrary.RandomFloatInRange` 0.0 1.0)) :!label _label_4)
      (`NiagaraComponent.SetVariableFloat` _ns_shield_sphere "SpawnRate01" 30.0)
      (`NiagaraComponent.SetVariableFloat` _ns_shield_sphere "SpawnRate02" 50.0))
    (:`P`
      (goto _label_4))
    (:`E`
      (goto _label_4))))