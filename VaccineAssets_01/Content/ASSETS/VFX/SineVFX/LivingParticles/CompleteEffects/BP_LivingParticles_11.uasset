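; Living particles VFX actor that feeds affector actor positions to a render target, presumably for its particle effect to read.
; On BeginPlay it adds the player character if the first affector is invalid.
; Each tick it redraws PositionsTexture, writing one pixel per affector in 16-wide rows, with position in RGB and affector count in alpha.
; Positions include a configurable offset and are actor-relative (translation only) unless GPUCPUOffsetEnabled is set.
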(event `self.ReceiveBeginPlay`
  (`/Engine/EditorBlueprintResources/StandardMacros.IsValid` (`|GetArrayItem` (`self.Affectors`))
    (:`Is Not Valid`
      (`KismetArrayLibrary.Array_Add` (`self.Affectors`) (`GameplayStatics.GetPlayerCharacter` 0)))))

(event `self.ReceiveTick`
  (params (DeltaSeconds :type "Float (single-precision)"))
  (bind _positionstexture (`self.PositionsTexture`))
  (bind _affectors (`self.Affectors`))
  (if (`self.GPUCPUOffsetEnabled`)
    (set `self.GPUCPUOffset` (0.0 0.0 0.0))
    (else
      (set `self.GPUCPUOffset` (`KismetMathLibrary.NegateVector` (`self.K2_GetActorLocation`)))))
  (`KismetRenderingLibrary.ClearRenderTarget2D` _positionstexture)
  (bind (_canvas _size _context) (`KismetRenderingLibrary.BeginDrawCanvasToRenderTarget` _positionstexture))
  (for (_array_element _array_index) _affectors
    (bind _returnvalue (`KismetMathLibrary.Conv_IntToDouble` (`KismetMathLibrary.FFloor` (/ (`KismetMathLibrary.Conv_IntToDouble` _array_index) 16.0))))
    (`Canvas.K2_DrawTexture` _canvas null (`KismetMathLibrary.MakeVector2D` (- (`KismetMathLibrary.Conv_IntToDouble` _array_index) (* 16.0 _returnvalue)) _returnvalue) (1.0 1.0) (0.0 0.0) (1.0 1.0) (`KismetMathLibrary.MakeColor` (.x (+ (`self.K2_GetActorLocation` _array_element) (`self.GPUCPUOffset`) (`self.AffectorsPositionOffset`))) (.y (+ (`self.K2_GetActorLocation` _array_element) (`self.GPUCPUOffset`) (`self.AffectorsPositionOffset`))) (.z (+ (`self.K2_GetActorLocation` _array_element) (`self.GPUCPUOffset`) (`self.AffectorsPositionOffset`))) (`KismetMathLibrary.Conv_IntToDouble` (`KismetArrayLibrary.Array_Length` _affectors))) "BLEND_Opaque" 0.0 (0.5 0.5)))
  (`KismetRenderingLibrary.EndDrawCanvasToRenderTarget` _context))

(fn `UserConstructionScript`)