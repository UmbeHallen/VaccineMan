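; Demo controller actor that cycles through the LivingParticles complete effects, showing one spawned effect at a time.
; On BeginPlay it enables player input and spawns the current entry of the CompleteEffects class array at the world origin.
; Q and E step the index back and forward with hard-coded wraparound; E wraps upon reaching 27, so only Q lands on that index.
; Each switch spawns the new effect and destroys the previous one.
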(event `Key|Q`
  (params (Key :type "Key Structure"))
  (:`Pressed`
    (bind _output_get (set `self.CurrentEffectInt` (+ (`self.CurrentEffectInt`) (* (`self.Int`) -1))))
    (`/Engine/EditorBlueprintResources/StandardMacros.CompareInt` _output_get -1
      (:`>`
        _)
      (:`==`
        (set `self.CurrentEffectInt` 27))
      (:`<`
        _))
    (bind _returnvalue (`|SpawnActorFromClass` (`|GetArrayItem` (`self.CompleteEffects`) (`self.CurrentEffectInt`)) (`KismetMathLibrary.MakeTransform` (0.0 0.0 0.0)) "Undefined" "OverrideRootScale" null null :!label _label))
    (`/Engine/EditorBlueprintResources/StandardMacros.IsValid` (`self.CurrentEffect`)
      (:`Is Valid`
        (set `self.PreviousEffect` (`self.CurrentEffect`))
        (set `self.CurrentEffect` _returnvalue)
        (`self.K2_DestroyActor` (`self.PreviousEffect`)))
      (:`Is Not Valid`
        (set `self.CurrentEffect` _returnvalue)))))

(event `Key|E`
  (params (Key :type "Key Structure"))
  (:`Pressed`
    (bind _output_get (set `self.CurrentEffectInt` (+ (`self.CurrentEffectInt`) (`self.Int`))))
    (`/Engine/EditorBlueprintResources/StandardMacros.CompareInt` _output_get 27
      (:`>`
        (goto _label))
      (:`==`
        (set `self.CurrentEffectInt` 0)
        (goto _label))
      (:`<`
        (goto _label)))))

(event `self.ReceiveBeginPlay`
  (`self.EnableInput` (`GameplayStatics.GetPlayerController` 0))
  (goto _label))

(fn `UserConstructionScript`)