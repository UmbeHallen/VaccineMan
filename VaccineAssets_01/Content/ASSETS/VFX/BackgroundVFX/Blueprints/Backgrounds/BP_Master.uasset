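; BP_Master is a configurable pawn that presents a mouse-reactive VFX background scene with a UI widget on top.
; The construction script applies options for planes, camera, Niagara template, post process and light.
; BeginPlay handles fade, cursor, widget, possession and delayed time dilation.
; Tick optionally sways the camera toward the mouse, and feeds MouseLocation to a material parameter collection via line trace and to Niagara via cursor direction.
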(event `Key|SpaceBar`
  (params (Key :type "Key Structure"))
  (:`Pressed`
    (`AutomationBlueprintFunctionLibrary.TakeHighResScreenshot` 1920 1080 (`KismetStringLibrary.Concat_StrStr` "Screenshot" (`KismetStringLibrary.Conv_DoubleToString` (`KismetMathLibrary.RandomFloatInRange` 0.0 100.0))) null)))

(event `self.ReceiveBeginPlay`
  (bind _returnvalue (`GameplayStatics.GetPlayerController` 0))
  ;[1 0.2707 0 0.1] BeginPlay
  (`|ExecutionSequence`
    (:`then_0`
      (if (`self.UseFade?`)
        (`PlayerCameraManager.StartCameraFade` (`GameplayStatics.GetPlayerCameraManager` 0) (`self.FadeStartAlpha`) 0.0 (`self.FadeDuration`) (`self.FadeColor`) true false))
      (set `PlayerController.bShowMouseCursor` true _returnvalue)
      (bind _returnvalue_2 (`|CreateWidget` (`self.Widget`)))
      (`UserWidget.AddToViewport` _returnvalue_2 0))
    (:`then_1`
      (`Controller.Possess` _returnvalue self)
      (`self.EnableInput` self _returnvalue))
    (:`then_2`
      (`KismetSystemLibrary.Delay` (`self.TimeDilationDelay`))
      (if (`self.UseTimeDilation?`)
        (`GameplayStatics.SetGlobalTimeDilation` (`self.TimeDilation`))))))

(event `self.ReceiveTick`
  (params (DeltaSeconds :type "Float (single-precision)"))
  (bind _maxsway (`self.MaxSway`))
  (bind _camera (`self.Camera`))
  (bind (_worldlocation _worlddirection) (`PlayerController.DeprojectMousePositionToWorld` (`GameplayStatics.GetPlayerController` 0)))
  (bind (_returnvalue_roll _returnvalue_pitch _returnvalue_yaw) (`KismetMathLibrary.BreakRotator` (`KismetMathLibrary.FindLookAtRotation` (`SceneComponent.K2_GetComponentLocation` _camera) _worldlocation)))
  ;[0 0 0] Tick
  (`|ExecutionSequence`
    (:`then_0`
      (if (`self.UseMouseSway?`)
        (`SceneComponent.K2_SetRelativeRotation` _camera (`KismetMathLibrary.RInterpTo` (`SceneComponent.RelativeRotation` _camera) (`KismetMathLibrary.MakeRotator` 0.0 (`KismetMathLibrary.FClamp` _returnvalue_pitch 0.0 _maxsway) (`KismetMathLibrary.FClamp` _returnvalue_yaw 0.0 _maxsway)) DeltaSeconds (`self.SwaySpeed`)) false false)))
    (:`then_1`
      (bind _outhit (`KismetSystemLibrary.LineTraceSingle` :`Start` _worldlocation :`End` (+ (* _worlddirection 1000) _worldlocation) :`TraceChannel` "TraceTypeQuery1" :`bIgnoreSelf` false))
      (`KismetMaterialLibrary.SetVectorParameterValue` "/Game/ASSETS/VFX/BackgroundVFX/Materials/CollectionParameters/MPC_Master.MPC_Master" "MouseLocation" (`KismetMathLibrary.Conv_VectorToLinearColor` (`.Location` (`GameplayStatics.BreakHitResult` _outhit)))))
    (:`then_2`
      (`FXSystemComponent.SetVectorParameter` (`self.Niagara`) "MouseLocation" (`KismetMathLibrary.MakeVector` 0.0 (.x _worlddirection) (.y _worlddirection))))))

(fn `UserConstructionScript`
  (bind _plane1 (`self.Plane1`))
  (bind _pointlight (`self.PointLight`))
  (bind _plane (`self.Plane`))
  (`|ExecutionSequence`
    (:`then_0`
      (if (`self.UseBackgroundPlane?`)
        (`SceneComponent.SetVisibility` _plane true false)
        (`PrimitiveComponent.SetMaterial` _plane 0 (`self.PlaneMaterial`))
        (if (`self.UseSecondPlane?`)
          (`SceneComponent.SetVisibility` _plane1 true false)
          (`PrimitiveComponent.SetMaterial` _plane1 0 (`self.SecondPlaneMaterial`))
          (else
            (`SceneComponent.SetVisibility` _plane1 false false :!label _label)))
        (else
          (`SceneComponent.SetVisibility` _plane false false)
          (goto _label))))
    (:`then_1`
      (`CameraComponent.SetFieldOfView` (`self.Camera`) (`self.FOV`))
      (if (`self.UseTimeDilation?`)
        (`GameplayStatics.SetGlobalTimeDilation` (`self.TimeDilation`))))
    (:`then_2`
      (`NiagaraComponent.SetAsset` (`self.Niagara`) (`self.NiagaraTemplate`) true))
    (:`then_3`
      (if (`self.UsePostProcessSettings?`)
        (set `CameraComponent.PostProcessSettings` (`self.PostProcessSettings`) (`self.Camera`))))
    (:`then_4`
      (if (`self.UseLight?`)
        (`SceneComponent.SetVisibility` _pointlight true false)
        (`LightComponent.SetIntensity` _pointlight (`self.LightIntensity`))
        (`LightComponent.SetLightColor` _pointlight (`self.LightColor`) true)
        (`LocalLightComponent.SetAttenuationRadius` _pointlight (`self.LightRadius`))
        (else
          (`SceneComponent.SetVisibility` _pointlight false false))))))