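; Laser actor that burns damage into whatever surface its beam hits.
; Each tick it traces from the Arrow, stretches the laser mesh to the hit and spawns flash, hit and melting particles.
; First hits give objects their own render target, mapped by name and fed to a dynamic material as DamageRT.
; A brush material paints into that target at the hit's collision UV, with strength scaled by delta time.
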(event `self.ReceiveBeginPlay`
  ;[1 1 1] Create/Remove Brush
  (`KismetRenderingLibrary.ClearRenderTarget2D` "/Game/ASSETS/VFX/LaserDamageVFX/RenderTargets/RT_Damage.RT_Damage")
  (bind _returnvalue (`KismetMaterialLibrary.CreateDynamicMaterialInstance` "/Game/ASSETS/VFX/LaserDamageVFX/Materials/M_Brush.M_Brush"))
  (set `self.Brush` _returnvalue))

(event `self.ReceiveTick`
  (params (DeltaSeconds :type "Float (single-precision)"))
  (bind _nametort (`self.NameToRT`))
  (bind _brush (`self.Brush`))
  (bind _arrow (`self.Arrow`))
  (bind _returnvalue (`SceneComponent.K2_GetComponentLocation` _arrow))
  ;[1 1 1] LineTrace
  (bind (_outhit _returnvalue_2) (`KismetSystemLibrary.LineTraceSingle` _returnvalue (+ _returnvalue (* (`SceneComponent.GetForwardVector` _arrow) (`self.LaserLength`))) "TraceTypeQuery1" true))
  (if _returnvalue_2
    (bind (_bblockinghit _binitialoverlap _time _distance _location _impactpoint _normal _impactnormal _physmat _hitactor _hitcomponent _hitbonename _hititem _elementindex _faceindex _tracestart) (`GameplayStatics.BreakHitResult` _outhit))
    ;[1 1 1] SpawnLaserMesh
    (`SceneComponent.SetWorldScale3D` (`self.Laser`) (`KismetMathLibrary.MakeVector` 0.1 0.1 (/ (`KismetMathLibrary.Vector_Distance` _location _tracestart) 19.5)))
    ;[1 1 1] SpawnHitParticle
    (`SceneComponent.SetVisibility` (`self.Laser`) true false)
    (`ActorComponent.SetActive` (`self.Flash`) true false)
    (`GameplayStatics.SpawnEmitterAtLocation` "/Game/ASSETS/VFX/LaserDamageVFX/Particles/Hits/P_Hit_06.P_Hit_06" _location)
    (`GameplayStatics.SpawnEmitterAtLocation` "/Game/ASSETS/VFX/LaserDamageVFX/Particles/P_Melting_Red.P_Melting_Red" _location (struct :`Pitch` 180.0))
    (bind _returnvalue_3 (`KismetSystemLibrary.GetObjectName` _hitactor))
    ;[1 1 1] LaserDamage
    (if (not (`BlueprintMapLibrary.Map_Contains` _nametort _returnvalue_3))
      (bind _returnvalue_4 (`KismetRenderingLibrary.CreateRenderTarget2D` 1024 1024))
      (`BlueprintMapLibrary.Map_Add` _nametort _returnvalue_3 _returnvalue_4)
      (bind _returnvalue_5 (`KismetMaterialLibrary.CreateDynamicMaterialInstance` (`PrimitiveComponent.GetMaterial` _hitcomponent 0)))
      (`PrimitiveComponent.SetMaterial` _hitcomponent 0 _returnvalue_5)
      (`MaterialInstanceDynamic.SetTextureParameterValue` _returnvalue_5 "DamageRT" _returnvalue_4))
    (`MaterialInstanceDynamic.SetVectorParameterValue` _brush "UVLoc" (`KismetMathLibrary.Conv_VectorToLinearColor` (`KismetMathLibrary.Conv_Vector2DToVector` (`GameplayStatics.FindCollisionUV` _outhit))))
    (`MaterialInstanceDynamic.SetScalarParameterValue` _brush "ForceStrength" (* (`GameplayStatics.GetWorldDeltaSeconds`) (`self.BrushStrength`)))
    (`MaterialInstanceDynamic.SetScalarParameterValue` _brush "Size" (`self.BrushSize`))
    (`KismetRenderingLibrary.DrawMaterialToRenderTarget` (`BlueprintMapLibrary.Map_Find` (`self.NameToRT`) _returnvalue_3) _brush)))

(fn `UserConstructionScript`)