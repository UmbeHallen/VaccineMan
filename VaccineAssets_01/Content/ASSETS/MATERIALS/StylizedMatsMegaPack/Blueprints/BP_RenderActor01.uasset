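; BP_RenderActor01 is a material showcase actor that cycles its render sphere mesh through the Mats array during play.
; From BeginPlay, it waits Period seconds, applies the Current material to slot 0, advances the index with wraparound, and re-enters the delay through a custom update event to loop.
; The construction script applies the material at the Preview index, if valid, as an editor preview.
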(event `self.ReceiveBeginPlay`
  (bind _mats (`self.Mats`))
  ;[1 1 1] MaterialUpdateLoop
  (set `self.Length` (- (`KismetArrayLibrary.Array_Length` _mats) 1))
  (`KismetSystemLibrary.Delay` (`self.Period`) :!label _label)
  (`PrimitiveComponent.SetMaterial` (`self.SM_RenderSphere01`) 0 (`|GetArrayItem` _mats (`self.Current`)))
  (bind _output_get (set `self.Current` (+ (`self.Current`) 1)))
  (if (> _output_get (`self.Length`))
    (set `self.Current` 0)
    (`self.CE_Update`)
    (else
      (`self.CE_Update`))))

(event `CE_Update`
  ;[1 1 1] MaterialUpdateLoop
  (goto _label))

(fn `UserConstructionScript`
  (bind _output (`|GetArrayItem` (`self.Mats`) (`self.Preview`)))
  (`/Engine/EditorBlueprintResources/StandardMacros.IsValid` _output
    (:`Is Valid`
      (`PrimitiveComponent.SetMaterial` (`self.SM_RenderSphere01`) 0 _output))))