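; BP_USEnemy2 is an enemy actor for UnderSiege that moves in a straight line and can be destroyed.
; Each Tick offsets the root along local Y by USSpeed, without delta-time scaling.
; When USEnemyHealth, which this graph only reads, drops below zero, it spawns BP_USExplode_1 at the mesh location and destroys itself.
; A BeginPlay delay also removes it silently after AbsLifeTime.
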(event `self.ReceiveBeginPlay`
  (`KismetSystemLibrary.Delay` (`self.AbsLifeTime`))
  (`self.K2_DestroyActor`))

(event `self.ReceiveTick`
  (params (DeltaSeconds :type "Float (single-precision)"))
  (`SceneComponent.K2_AddLocalOffset` (`self.DefaultSceneRoot`) (`KismetMathLibrary.MakeVector` 0.0 (`self.USSpeed`)) false false)
  (if (< (`self.USEnemyHealth`) 0.0)
    (`|SpawnActorFromClass` "/Game/ASSETS/CODE/UnderSiege/BluePrints/System/BP_USExplode_1.BP_USExplode_1_C" (`KismetMathLibrary.MakeTransform` (`SceneComponent.K2_GetComponentLocation` (`self.SM_enemy_2`))) "AlwaysSpawn" "OverrideRootScale" null null)
    (`self.K2_DestroyActor`)))

(fn `UserConstructionScript`)