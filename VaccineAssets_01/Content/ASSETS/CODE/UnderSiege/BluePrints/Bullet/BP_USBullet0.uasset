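; BP_USBullet0 is an UnderSiege laser projectile that notifies the player pawn when it hits it.
; Tick sweeps LaserBullet along local Y by Speed, without delta-time scaling, and BeginPlay destroys the actor after AbsLifeTime.
; Any hit destroys it, first sending ToPlayerMessage if the target is the player.
; Enemy damage logic is disconnected, and InfoToUI returns only zeros.
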(event `self.ReceiveBeginPlay`
  (`KismetSystemLibrary.Delay` (`self.AbsLifeTime`))
  (`self.K2_DestroyActor`))

(event `self.ReceiveTick`
  (params (DeltaSeconds :type "Float (single-precision)"))
  (`SceneComponent.K2_AddLocalOffset` (`self.laser_bullet`) (`KismetMathLibrary.MakeVector` 0.0 (`self.Speed`)) true false))

(event `self.ReceiveHit`
  (params (MyComp :type "PrimitiveComponent Object Reference") (Other :type "Actor Object Reference") (OtherComp :type "PrimitiveComponent Object Reference") (bSelfMoved :type Boolean) (HitLocation :type "Vector Structure") (HitNormal :type "Vector Structure") (NormalImpulse :type "Vector Structure") (Hit :type "HitResult Structure (by ref)"))
  (if (== (`GameplayStatics.GetPlayerPawn` 0) Other)
    (message `/Game/GAME_FOLDER/CORE/UTILITY/Main_Interface.To_Player` Other "NewEnumerator0"))
  (`self.K2_DestroyActor`))

(fn `Info_To_UI`
  (returns (Speed_level :type Integer) (Resistance_Level :type Integer) (Dmg_level :type Integer) (Curretn_Resistance :type Integer))
  (return 0 0 0 0))

(fn `UserConstructionScript`)