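; BP_USRadar is an UnderSiege radar part whose rotor spins continuously about its local yaw axis.
; On BeginPlay it picks a random speed and direction, with the integer roll favoring negative spin two to one.
; Tick adds that speed as local rotation to the rotor component without delta-time scaling, so spin rate depends on frame rate.
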(event `self.ReceiveBeginPlay`
  (if (> (`KismetMathLibrary.RandomIntegerInRange` -1 1) 0)
    (set `self.SpeedRot` (`KismetMathLibrary.RandomFloatInRange` 1.0 5.0))
    (else
      (set `self.SpeedRot` (`KismetMathLibrary.RandomFloatInRange` -1.0 -5.0)))))

(event `self.ReceiveTick`
  (params (DeltaSeconds :type "Float (single-precision)"))
  (`SceneComponent.K2_AddLocalRotation` (`self.radar_radar_rotor`) (`KismetMathLibrary.MakeRotator` 0.0 0.0 (`self.SpeedRot`)) false false))

(fn `UserConstructionScript`)