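; BP_USFlowSpawner is an UnderSiege spawner that keeps adding child actors at random positions on its local XZ plane.
; A one-time, one-second delay on Tick uses a FlipFlop to set the flag that starts spawning.
; Each active Tick then randomizes its own interval within the configured range, and a looping random MultiGate picks one of two AddChildActorComponent branches, both placing within configurable X and Z bounds.
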(event `self.ReceiveTick`
  (params (DeltaSeconds :type "Float (single-precision)"))
  (bind _returnvalue (`KismetMathLibrary.MakeTransform` (`KismetMathLibrary.MakeVector` (`KismetMathLibrary.RandomFloatInRange` (`self.XMin`) (`self.XMax`)) 0.0 (`KismetMathLibrary.RandomFloatInRange` (`self.ZMin`) (`self.ZMax`)))))
  (if (stale _isa)
    (`self.SetActorTickInterval` (`KismetMathLibrary.RandomFloatInRange` (`self.SpawnIntervalMin`) (`self.SpawnIntervalMax`)))
    (`|MultiGate` true true 2
      (:`Out 0`
        (`AddComponent|NODE_AddChildActorComponent-1` :`RelativeTransform` _returnvalue))
      (:`Out 1`
        (`AddComponent|NODE_AddChildActorComponent-2` :`RelativeTransform` _returnvalue)))
    (else
      (`/Engine/EditorBlueprintResources/StandardMacros.DoOnce` false
        (:`Completed`
          (`KismetSystemLibrary.Delay` 1.0)
          (bind _isa (`/Engine/EditorBlueprintResources/StandardMacros.FlipFlop`)))))))

(fn `UserConstructionScript`)