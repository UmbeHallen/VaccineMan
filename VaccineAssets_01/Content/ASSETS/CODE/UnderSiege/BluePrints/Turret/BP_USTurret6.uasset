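; Auto-aiming Under Siege turret, floor-mounted or inverted via DownTurret, with a shield-sphere hit effect.
; Tick picks a random response-area target, waits a ready time, then interpolates yaw and pitch toward targets on its facing side while ramping gun emissive.
; A Delay in Tick paces animated BP_USBullet0 shots.
; Shield hits drive Niagara and material ripples through a timeline, calling the empty OnTakingDmg stub each update.
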(event `self.ReceiveBeginPlay`
  (bind _defaultsceneroot (`self.DefaultSceneRoot`))
  (`PrimitiveComponent.CreateDynamicMaterialInstance` (`self.SK_turret3_gun`) 0 null "None")
  (if (`self.DownTurret`)
    (`SceneComponent.K2_SetWorldRotation` _defaultsceneroot (struct :`Pitch` 180.0 :`Yaw` 180.0 :`Roll` 180.0) false false)
    (`SceneComponent.K2_SetWorldRotation` (`self.SM_turret3_base_head`) (struct :`Pitch` 180.0) false false)
    (`SceneComponent.K2_SetWorldRotation` (`self.SM_turret3_base_rot_yaw`) (struct :`Pitch` 180.0) false false)
    (else
      (`SceneComponent.K2_SetWorldRotation` :`self` _defaultsceneroot))))

(event `self.ReceiveTick`
  (params (DeltaSeconds :type "Float (single-precision)"))
  (bind (_returnvalue_x _returnvalue_y _returnvalue_z) (`KismetMathLibrary.BreakVector` (`self.K2_GetActorLocation`)))
  (bind (_returnvalue_x_2 _returnvalue_y_2 _returnvalue_z_2) (`KismetMathLibrary.BreakVector` (`self.K2_GetActorLocation`)))
  (bind _sk_turret3_gun (`self.SK_turret3_gun`))
  (bind _sk_turret3_gun_2 (`self.SK_turret3_gun`))
  (bind _materiallerp_x (`KismetMathLibrary.BreakVector` (`self.MaterialLerp`)))
  (bind _sk_turret3_gun_3 (`self.SK_turret3_gun`))
  (bind (_returnvalue_x_3 _returnvalue_y_3 _returnvalue_z_3) (`KismetMathLibrary.BreakVector` (`SceneComponent.K2_GetComponentLocation` _sk_turret3_gun_2)))
  (bind _returnvalue_x_4 (`KismetMathLibrary.BreakVector` (`KismetMathLibrary.VInterpTo` (`self.MaterialLerp`) (0.0 0.0 0.0) (`GameplayStatics.GetWorldDeltaSeconds`) 0.7)))
  (bind _returnvalue_x_5 (`KismetMathLibrary.BreakVector` (`KismetMathLibrary.VInterpTo` (`self.MaterialLerp`) (14.0 0.0 0.0) (`GameplayStatics.GetWorldDeltaSeconds`) 0.02)))
  (bind _usresponsearearef (`self.USResponseAreaRef`)
    (:`then`
      (if (`self.IsAim`)
        (bind _usresponseareatargets (`/Game/ASSETS/CODE/UnderSiege/BluePrints/System/BP_USResponseArea.USResponseAreaTargets` _usresponsearearef))
        (bind _output (`|GetArrayItem` _usresponseareatargets (`self.TargetOffset`)))
        (bind _returnvalue (`KismetSystemLibrary.IsValid` _output))
        (if _returnvalue
          (if (`self.IsReady`)
            (bind (_returnvalue_x_6 _returnvalue_y_4 _returnvalue_z_4) (`KismetMathLibrary.BreakVector` (`self.K2_GetActorLocation` _output)))
            (bind (_returnvalue_x_7 _returnvalue_y_5 _returnvalue_z_5) (`KismetMathLibrary.BreakVector` (`self.K2_GetActorLocation` _output)))
            (if (or (and (not (`self.DownTurret`)) (> _returnvalue_z_4 _returnvalue_z)) (and (`self.DownTurret`) (< _returnvalue_z_5 _returnvalue_z_2)))
              (`MeshComponent.SetScalarParameterValueOnMaterials` (`self.SK_turret3_gun`) "EmissiveMP" _returnvalue_x_5)
              (set `self.MaterialLerp` (`KismetMathLibrary.Conv_DoubleToVector` _returnvalue_x_5))
              (bind (_returnvalue_roll _returnvalue_pitch _returnvalue_yaw) (`KismetMathLibrary.BreakRotator` (`KismetMathLibrary.FindLookAtRotation` (`self.K2_GetActorLocation`) (`self.K2_GetActorLocation` _output))))
              (`SceneComponent.K2_SetRelativeRotation` (`self.SM_turret3_base_rot_yaw`) (`KismetMathLibrary.RInterpTo` (`SceneComponent.K2_GetComponentRotation` (`self.SM_turret3_base_rot_yaw`)) (`KismetMathLibrary.MakeRotator` 0.0 0.0 _returnvalue_yaw) (`GameplayStatics.GetWorldDeltaSeconds`) (`self.YawAimSpeed`)) false false)
              (`SceneComponent.K2_SetRelativeRotation` _sk_turret3_gun_3 (`KismetMathLibrary.RInterpTo` (`SceneComponent.RelativeRotation` _sk_turret3_gun_3) (`KismetMathLibrary.MakeRotator` 0.0 _returnvalue_pitch) (`GameplayStatics.GetWorldDeltaSeconds`) (`self.PitchAimSpeed`)) false false)
              (`SceneComponent.K2_SetRelativeRotation` (`self.MaxRotation`) (`KismetMathLibrary.RInterpTo` (`SceneComponent.RelativeRotation` (`self.MaxRotation`)) (`KismetMathLibrary.MakeRotator` _returnvalue_roll) (`GameplayStatics.GetWorldDeltaSeconds`) (`self.PitchAimSpeed`)) false false)
              (`KismetSystemLibrary.Delay` (`self.FireRate`))
              (`SkeletalMeshComponent.PlayAnimation` _sk_turret3_gun "/Game/ASSETS/CODE/UnderSiege/Animations/Anim_turret3_gun_Anim.Anim_turret3_gun_Anim" false)
              (`SkeletalMeshComponent.SetPlayRate` _sk_turret3_gun (`self.GunAnimRate`))
              (`|SpawnActorFromClass` "/Game/ASSETS/CODE/UnderSiege/BluePrints/Bullet/BP_USBullet0.BP_USBullet0_C" (`KismetMathLibrary.MakeTransform` (`KismetMathLibrary.MakeVector` _returnvalue_x_3 _returnvalue_y_3 (+ _returnvalue_z_3 7.0)) (`SceneComponent.K2_GetComponentRotation` _sk_turret3_gun_2)) "AlwaysSpawn" "OverrideRootScale" null null))
            (else
              (`KismetSystemLibrary.Delay` (`self.ReadyTime`))
              (set `self.IsReady` true)))
          (else
            (set `self.IsAim` false)
            (set `self.IsReady` false)))
        (else
          (set `self.TargetOffset` (`KismetMathLibrary.RandomIntegerInRange` 0 (- (`KismetArrayLibrary.Array_Length` _usresponseareatargets) 1)))
          (if _returnvalue
            (set `self.IsAim` true)
            (elif (> _materiallerp_x 0.0)
              (`MeshComponent.SetScalarParameterValueOnMaterials` (`self.SK_turret3_gun`) "EmissiveMP" _returnvalue_x_4)
              (set `self.MaterialLerp` (`KismetMathLibrary.Conv_DoubleToVector` _returnvalue_x_4)))))))
    (:`else`)))

(event `SetUpTurret`)

(event `self.SM_Sphere.OnComponentHit`
  (params (HitComponent :type "PrimitiveComponent Object Reference") (OtherActor :type "Actor Object Reference") (OtherComp :type "PrimitiveComponent Object Reference") (NormalImpulse :type "Vector Structure") (Hit :type "HitResult Structure (by ref)"))
  ;[1 1 1 1 30] HIT EFFECT
  ;;[1 1 1] Niagara
  (`NiagaraComponent.SetVariableVec3` (`self.NS_Shield_Sphere`) "Hit_SphereLocation" Hit_ImpactPoint)
  ;;[1 1 1] Mesh
  (bind _returnvalue (`PrimitiveComponent.CreateDynamicMaterialInstance` (`self.SM_Sphere`) 0 "/Game/ASSETS/VFX/Shield_FX_Niagara/Niagara_Shield/Material/M_waterDrop.M_waterDrop" "None"))
  (`MaterialInstanceDynamic.SetVectorParameterValue` _returnvalue "Hit_Location" (`KismetMathLibrary.Conv_VectorToLinearColor` Hit_ImpactPoint))
  (`NiagaraFunctionLibrary.SpawnSystemAtLocation` "/Game/ASSETS/VFX/Shield_FX_Niagara/Hit_Particles/NS_Hit_Bubble.NS_Hit_Bubble" Hit_ImpactPoint (`KismetMathLibrary.MakeRotFromZ` Hit_ImpactNormal))
  (bind (_direction _vertexnoise_strength _hit_opacity _radius_hit _vertexnoise_radius _niagara_hit_radius) (`Timeline|Timeline_0` :!via `PlayFromStart`)
    (:`Update`
      (`NiagaraComponent.SetVariableFloat` (`self.NS_Shield_Sphere`) "Hit_SphereRadius" (* _niagara_hit_radius (`self.Niagara_Hit_Radius`)))
      (`MaterialInstanceDynamic.SetScalarParameterValue` _returnvalue "Radius_VertexNoise" (* _vertexnoise_radius (`self.Radius_VertexNoise`)))
      (`MaterialInstanceDynamic.SetScalarParameterValue` _returnvalue "Strength_VertexNoise" (* _vertexnoise_strength (`self.VertexNoise_Strength`)))
      (`MaterialInstanceDynamic.SetScalarParameterValue` _returnvalue "Hit_opacity" _hit_opacity)
      (`MaterialInstanceDynamic.SetScalarParameterValue` _returnvalue "radius_Hit" (* _radius_hit (`self.radius_Hit`) 0.0))
      (`self.OnTakingDmg`))))

(event `CustomEvent`)

(fn `OnTakingDmg`)

(fn `UserConstructionScript`)