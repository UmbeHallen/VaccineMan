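; BP_USTurret3 is an automatic turret that fires BP_USBullet3 at targets from a response area, mountable upright or inverted via DownTurret.
; Tick picks a random target, keeps it while valid, and waits ReadyTime before engaging.
; For targets on its facing side, it interpolates base yaw and gun pitch, using Delay inside Tick to pace firing.
; An emissive material parameter ramps up while engaging and fades without a target.
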(event `self.ReceiveBeginPlay`
  (bind _defaultsceneroot (`self.DefaultSceneRoot`))
  (`PrimitiveComponent.CreateDynamicMaterialInstance` (`self.SK_turret3_gun`) 0 null "None")
  (if (`self.DownTurret`)
    (`SceneComponent.K2_SetWorldRotation` _defaultsceneroot (struct :`Pitch` 180.0 :`Yaw` 180.0 :`Roll` 180.0) false false)
    (`SceneComponent.K2_SetWorldRotation` (`self.SM_turret3_base_head`) (struct :`Pitch` 180.0) false false)
    (`SceneComponent.K2_SetWorldRotation` (`self.SM_turret3_base_rot_yaw`) (struct :`Pitch` 180.0) false false)
    (else
      (`SceneComponent.K2_SetWorldRotation` :`self` _defaultsceneroot))))

(event `self.ReceiveTick`
  (params (DeltaSeconds :type "Float (single-precision)"))
  (bind (_returnvalue_x _returnvalue_y _returnvalue_z) (`KismetMathLibrary.BreakVector` (`self.K2_GetActorLocation`)))
  (bind (_returnvalue_x_2 _returnvalue_y_2 _returnvalue_z_2) (`KismetMathLibrary.BreakVector` (`self.K2_GetActorLocation`)))
  (bind _sk_turret3_gun (`self.SK_turret3_gun`))
  (bind _downturret (`self.DownTurret`))
  (bind _sk_turret3_gun_2 (`self.SK_turret3_gun`))
  (bind _materiallerp_x (`KismetMathLibrary.BreakVector` (`self.MaterialLerp`)))
  (bind _sk_turret3_gun_3 (`self.SK_turret3_gun`))
  (bind (_returnvalue_x_3 _returnvalue_y_3 _returnvalue_z_3) (`KismetMathLibrary.BreakVector` (`SceneComponent.K2_GetComponentLocation` _sk_turret3_gun_2)))
  (bind _returnvalue_x_4 (`KismetMathLibrary.BreakVector` (`KismetMathLibrary.VInterpTo` (`self.MaterialLerp`) (0.0 0.0 0.0) (`GameplayStatics.GetWorldDeltaSeconds`) 0.7)))
  (bind _returnvalue_x_5 (`KismetMathLibrary.BreakVector` (`KismetMathLibrary.VInterpTo` (`self.MaterialLerp`) (14.0 0.0 0.0) (`GameplayStatics.GetWorldDeltaSeconds`) 0.02)))
  (bind _usresponsearearef (`self.USResponseAreaRef`)
    (:`then`
      (if (`self.IsAim`)
        (bind _usresponseareatargets (`/Game/ASSETS/CODE/UnderSiege/BluePrints/System/BP_USResponseArea.USResponseAreaTargets` _usresponsearearef))
        (bind _output (`|GetArrayItem` _usresponseareatargets (`self.TargetOffset`)))
        (bind _returnvalue (`KismetSystemLibrary.IsValid` _output))
        (if _returnvalue
          (if (`self.IsReady`)
            (bind (_returnvalue_x_6 _returnvalue_y_4 _returnvalue_z_4) (`KismetMathLibrary.BreakVector` (`self.K2_GetActorLocation` _output)))
            (bind (_returnvalue_x_7 _returnvalue_y_5 _returnvalue_z_5) (`KismetMathLibrary.BreakVector` (`self.K2_GetActorLocation` _output)))
            (if (or (and (not (`self.DownTurret`)) (> _returnvalue_z_4 _returnvalue_z_2)) (and (`self.DownTurret`) (< _returnvalue_z_5 _returnvalue_z)))
              (`MeshComponent.SetScalarParameterValueOnMaterials` (`self.SK_turret3_gun`) "EmissiveMP" _returnvalue_x_5)
              (set `self.MaterialLerp` (`KismetMathLibrary.Conv_DoubleToVector` _returnvalue_x_5))
              (bind (_returnvalue_roll _returnvalue_pitch _returnvalue_yaw) (`KismetMathLibrary.BreakRotator` (`KismetMathLibrary.FindLookAtRotation` (`self.K2_GetActorLocation`) (`self.K2_GetActorLocation` _output))))
              (`SceneComponent.K2_SetRelativeRotation` (`self.SM_turret3_base_rot_yaw`) (`KismetMathLibrary.RInterpTo` (`SceneComponent.K2_GetComponentRotation` (`self.SM_turret3_base_rot_yaw`)) (`KismetMathLibrary.MakeRotator` (select `bool` _downturret :`true` 180.0 :!type "Float (single-precision)") 0.0 (+ _returnvalue_yaw (select `bool` _downturret :`false` -90.0 :`true` 90.0 :!type "Float (single-precision)"))) (`GameplayStatics.GetWorldDeltaSeconds`) (`self.YawAimSpeed`)) false false)
              (`SceneComponent.K2_SetRelativeRotation` _sk_turret3_gun_3 (`KismetMathLibrary.RInterpTo` (`SceneComponent.RelativeRotation` _sk_turret3_gun_3) (`KismetMathLibrary.MakeRotator` (* _returnvalue_pitch (select `bool` _downturret :`false` -1.0 :`true` 1.0 :!type "Float (single-precision)"))) (`GameplayStatics.GetWorldDeltaSeconds`) (`self.PitchAimSpeed`)) false false)
              (`KismetSystemLibrary.Delay` (`self.FireRate`))
              (`SkeletalMeshComponent.PlayAnimation` _sk_turret3_gun "/Game/ASSETS/CODE/UnderSiege/Animations/Anim_turret3_gun_Anim.Anim_turret3_gun_Anim" false)
              (`SkeletalMeshComponent.SetPlayRate` _sk_turret3_gun (`self.GunAnimRate`))
              (`|SpawnActorFromClass` "/Game/ASSETS/CODE/UnderSiege/BluePrints/Bullet/BP_USBullet3.BP_USBullet3_C" (`KismetMathLibrary.MakeTransform` (`KismetMathLibrary.MakeVector` _returnvalue_x_3 _returnvalue_y_3 (+ _returnvalue_z_3 7.0)) (`SceneComponent.K2_GetComponentRotation` _sk_turret3_gun_2)) "AlwaysSpawn" "OverrideRootScale" null null))
            (else
              (`KismetSystemLibrary.Delay` (`self.ReadyTime`))
              (set `self.IsReady` true)))
          (else
            (set `self.IsAim` false)
            (set `self.IsReady` false)))
        (else
          (set `self.TargetOffset` (`KismetMathLibrary.RandomIntegerInRange` 0 (- (`KismetArrayLibrary.Array_Length` _usresponseareatargets) 1)))
          (if _returnvalue
            (set `self.IsAim` true)
            (elif (> _materiallerp_x 0.0)
              (`MeshComponent.SetScalarParameterValueOnMaterials` (`self.SK_turret3_gun`) "EmissiveMP" _returnvalue_x_4)
              (set `self.MaterialLerp` (`KismetMathLibrary.Conv_DoubleToVector` _returnvalue_x_4)))))))
    (:`else`)))

(fn `UserConstructionScript`)