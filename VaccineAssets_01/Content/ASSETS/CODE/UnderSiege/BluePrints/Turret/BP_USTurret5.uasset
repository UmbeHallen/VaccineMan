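; BP_USTurret5 is a laser turret that engages targets supplied by a response area, with DownTurret selecting an inverted mount.
; Each Tick it picks a random target, waits a ready time, then interpolates separate yaw and gun pitch toward targets on its facing vertical side.
; Delay nodes inside Tick pace firing, which spawns a laser bullet and briefly stretches a mesh to flash the beam.
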(event `self.ReceiveBeginPlay`
  (bind _defaultsceneroot (`self.DefaultSceneRoot`))
  (if (`self.DownTurret`)
    (`SceneComponent.K2_SetWorldRotation` _defaultsceneroot (struct :`Pitch` 180.0 :`Yaw` 180.0 :`Roll` 180.0) false false)
    (`SceneComponent.K2_SetWorldRotation` (`self.SM_turret5_base`) (struct :`Pitch` 180.0) false false)
    (`SceneComponent.K2_SetWorldRotation` (`self.SM_turret5_yawer`) (struct :`Pitch` 180.0) false false)
    (else
      (`SceneComponent.K2_SetWorldRotation` :`self` _defaultsceneroot)))
  (`SceneComponent.SetRelativeScale3D` (`self.SM_laser_bullet_scaled`) (0.0 0.0 0.0)))

(event `self.ReceiveTick`
  (params (DeltaSeconds :type "Float (single-precision)"))
  (bind (_returnvalue_x _returnvalue_y _returnvalue_z) (`KismetMathLibrary.BreakVector` (`self.K2_GetActorLocation`)))
  (bind (_returnvalue_x_2 _returnvalue_y_2 _returnvalue_z_2) (`KismetMathLibrary.BreakVector` (`self.K2_GetActorLocation`)))
  (bind _sm_laser_bullet_scaled (`self.SM_laser_bullet_scaled`))
  (bind _sm_turret5_gun (`self.SM_turret5_gun`))
  (bind _sm_turret5_gun_2 (`self.SM_turret5_gun`))
  (bind _downturret (`self.DownTurret`))
  (bind (_returnvalue_x_3 _returnvalue_y_3 _returnvalue_z_3) (`KismetMathLibrary.BreakVector` (`SceneComponent.K2_GetComponentLocation` _sm_turret5_gun_2)))
  (bind _usresponsearearef (`self.USResponseAreaRef`)
    (:`then`
      (if (`self.IsAim`)
        (bind _usresponseareatargets (`/Game/ASSETS/CODE/UnderSiege/BluePrints/System/BP_USResponseArea.USResponseAreaTargets` _usresponsearearef))
        (bind _output (`|GetArrayItem` _usresponseareatargets (`self.TargetOffset`)))
        (bind _returnvalue (`KismetSystemLibrary.IsValid` _output))
        (if _returnvalue
          (if (`self.IsReady`)
            (bind (_returnvalue_x_4 _returnvalue_y_4 _returnvalue_z_4) (`KismetMathLibrary.BreakVector` (`self.K2_GetActorLocation` _output)))
            (bind (_returnvalue_x_5 _returnvalue_y_5 _returnvalue_z_5) (`KismetMathLibrary.BreakVector` (`self.K2_GetActorLocation` _output)))
            (if (or (and (not (`self.DownTurret`)) (> _returnvalue_z_4 _returnvalue_z_2)) (and (`self.DownTurret`) (< _returnvalue_z_5 _returnvalue_z)))
              (bind (_returnvalue_roll _returnvalue_pitch _returnvalue_yaw) (`KismetMathLibrary.BreakRotator` (`KismetMathLibrary.FindLookAtRotation` (`self.K2_GetActorLocation`) (`self.K2_GetActorLocation` _output))))
              (`SceneComponent.K2_SetRelativeRotation` (`self.SM_turret5_yawer`) (`KismetMathLibrary.RInterpTo` (`SceneComponent.K2_GetComponentRotation` (`self.SM_turret5_yawer`)) (`KismetMathLibrary.MakeRotator` (select `bool` _downturret :`true` 180.0 :!type "Float (single-precision)") 0.0 (+ _returnvalue_yaw (select `bool` _downturret :`false` -90.0 :`true` 90.0 :!type "Float (single-precision)"))) (`GameplayStatics.GetWorldDeltaSeconds`) (`self.YawAimSpeed`)) false false)
              (`SceneComponent.K2_SetRelativeRotation` _sm_turret5_gun (`KismetMathLibrary.RInterpTo` (`SceneComponent.RelativeRotation` _sm_turret5_gun) (`KismetMathLibrary.MakeRotator` (* _returnvalue_pitch (select `bool` _downturret :`false` -1.0 :`true` 1.0 :!type "Float (single-precision)"))) (`GameplayStatics.GetWorldDeltaSeconds`) (`self.PitchAimSpeed`)) false false)
              (`KismetSystemLibrary.Delay` (`self.FireRate`))
              (`|SpawnActorFromClass` "/Game/ASSETS/CODE/UnderSiege/BluePrints/Bullet/BP_USBullet2_laser.BP_USBullet2_laser_C" (`KismetMathLibrary.MakeTransform` (`KismetMathLibrary.MakeVector` _returnvalue_x_3 _returnvalue_y_3 (+ _returnvalue_z_3 (select `bool` (`self.DownTurret`) :`false` -10.0 :`true` 7.0 :!type "Float (single-precision)"))) (`SceneComponent.K2_GetComponentRotation` _sm_turret5_gun_2)) "AlwaysSpawn" "OverrideRootScale" null null)
              (`SceneComponent.SetRelativeScale3D` _sm_laser_bullet_scaled (1.0 14000.0 1.0))
              (`KismetSystemLibrary.Delay` (`self.LineTime(Visual)`))
              (`SceneComponent.SetRelativeScale3D` _sm_laser_bullet_scaled (0.0 0.0 0.0)))
            (else
              (`KismetSystemLibrary.Delay` (`self.ReadyTime`))
              (set `self.IsReady` true)))
          (else
            (set `self.IsAim` false)
            (set `self.IsReady` false)))
        (else
          (set `self.TargetOffset` (`KismetMathLibrary.RandomIntegerInRange` 0 (- (`KismetArrayLibrary.Array_Length` _usresponseareatargets) 1)))
          (if _returnvalue
            (set `self.IsAim` true)))))
    (:`else`)))

(fn `UserConstructionScript`)