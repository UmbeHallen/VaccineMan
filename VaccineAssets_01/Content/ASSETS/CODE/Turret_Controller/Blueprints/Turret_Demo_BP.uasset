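; Demo turret pawn that the player aims with camera input and fires with the left mouse button.
; Left click spawns a Turret_Projectile_BP at the Emitter1 transform, with the turret as owner and instigator.
; Turn and LookUp axes feed the CameraControllerBP component, while holding right mouse toggles free camera rotation on TurretControllerBP.
; Pressing E hands possession to the first Turret_Demo2_BP found in the level.
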(event `Key|E`
  (params (Key :type "Key Structure"))
  ;[1 1 1] Swap Active Actor
  (:`Pressed`
    (bind _outactors (`GameplayStatics.GetAllActorsOfClass` "/Game/ASSETS/CODE/Turret_Controller/Blueprints/Turret_Demo2_BP.Turret_Demo2_BP_C"))
    (`Controller.Possess` (`GameplayStatics.GetPlayerController` 0) (`|GetArrayItem` _outactors))))

(event `Key|LeftMouseButton`
  (params (Key :type "Key Structure"))
  ;[1 1 1] Fire Projectile With Left Click
  (:`Pressed`
    (`|SpawnActorFromClass` "/Game/ASSETS/CODE/Turret_Controller/Blueprints/Turret_Projectile_BP.Turret_Projectile_BP_C" (`SceneComponent.K2_GetComponentToWorld` (`self.Emitter1`)) "Undefined" "OverrideRootScale" self self)))

(event `Key|RightMouseButton`
  (params (Key :type "Key Structure"))
  ;[1 1 1] Free Camera Rotation
  (:`Pressed`
    (set `self.Free Rotation` true)
    (`/Game/ASSETS/CODE/Turret_Controller/Blueprints/Turret_controller_BP.Free Camera Rotation` (`self.Turret_controller_BP`) (stale _output_get) :!label _label))
  (:`Released`
    (bind _output_get (set `self.Free Rotation` false))
    (goto _label)))

(event `InputAxis|Turn`
  (params (AxisValue :type "Float (single-precision)"))
  ;[1 1 1] Camera Inputs
  (`/Game/ASSETS/CODE/Turret_Controller/Blueprints/Camera_Controller_BP.Add look at direction (Camera)` (`self.Camera_Controller_BP`) AxisValue (stale `InputAxis|LookUp` AxisValue) :!label _label_2))

(event `InputAxis|LookUp`
  (params (AxisValue :type "Float (single-precision)"))
  ;[1 1 1] Camera Inputs
  (goto _label_2))

(fn `UserConstructionScript`)