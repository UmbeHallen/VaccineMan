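; Game mode Blueprint for the replicated turret setup that spawns a pawn for each connected player at match start.
; BeginPlay waits briefly so clients finish loading, avoiding missing pawns or failed possession, then loops over player indices.
; For each, it tries spawning the default pawn at successive PlayerStarts, using collision failure to skip occupied spots.
; The first successful spawn is possessed by that player's controller, and InitialGameStarted is set.
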(event `self.ReceiveBeginPlay`
  ;[1 1 1] Spawn players after giving them time to load in (letting them spawn "instantly" by default often was resulting in some clients not being given actors, and others not properly posessing their actors).
  (`KismetSystemLibrary.Delay` 2.0)
  ;[1 1 1] For eachp player, find a start and spawn a turret for them to possess (taken spots will result in an attempted spawn on a new spot).
  (bind _returnvalue (`self.GetNumPlayers`))
  (for _index (range _returnvalue)
    (bind _outactors (`GameplayStatics.GetAllActorsOfClass` "/Script/Engine.PlayerStart"))
    (for _array_element _outactors
      (bind _returnvalue_2 (`|SpawnActorFromClass` (`self.DefaultPawnClass`) (`self.GetTransform` _array_element) "AdjustIfPossibleButDontSpawnIfColliding" "OverrideRootScale" null null))
      (`/Engine/EditorBlueprintResources/StandardMacros.IsValid` _returnvalue_2
        (:`Is Valid`
          (`|ExecutionSequence`
            (:`then_0`
              (`Controller.Possess` (`GameplayStatics.GetPlayerController` _index) _returnvalue_2))
            (:`then_1`
              (break))))))
    (set `self.Initial Game Started` true)))

(fn `UserConstructionScript`)