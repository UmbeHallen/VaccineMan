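; Replicated turret demo pawn that handles camera look, free-rotation aiming and projectile firing, with a key to possess a Turret_Demo_BP actor.
; Mouse axes drive CameraControllerBP, while holding right click toggles free camera rotation on TurretControllerBP.
; Left click fires from each barrel the turret controller reports on target, skipping the optics slot.
; The server spawns projectiles directly; clients call a multicast spawn event instead.
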(event `Key|E`
  (params (Key :type "Key Structure"))
  ;[1 1 1] Swap Active Actor
  (:`Pressed`
    (bind _outactors (`GameplayStatics.GetAllActorsOfClass` "/Game/ASSETS/CODE/Turret_Controller/Blueprints/Turret_Demo_BP.Turret_Demo_BP_C"))
    (`Controller.Possess` (`GameplayStatics.GetPlayerController` 0) (`|GetArrayItem` _outactors))))

(event `self.ReceiveBeginPlay`
  ;[1 1 1] Create Barrels Array On Start
  (set `self.Main barrels array` (`|MakeArray` (`self.Emitter1`) null (`self.Emitter3`) (`self.Emitter4`))))

(event `Key|LeftMouseButton`
  (params (Key :type "Key Structure"))
  ;[1 1 1] Fire Projectile With Left Click
  (:`Pressed`
    (bind _output_get (set `self.cached pointed at array` (`/Game/ASSETS/CODE/Turret_Controller/Blueprints/Turret_controller_BP.Turret Pointed At Target` (`self.Turret_controller_BP`))))
    ;;[1 1 1] Spawn Projectiles Only If Barrel Is Pointed At Target
    (if (!= (`KismetArrayLibrary.Array_Length` _output_get) 0)
      (for (_array_element _array_index) (`self.Main barrels array`)
        ;;;[1 1 1] Exclude Optics From Firing
        (if (!= _array_index 1)
          ;;;[1 1 1] Spawn projectile on the server
          (if (`|GetArrayItem` (`self.cached pointed at array`) _array_index)
            (if (`KismetSystemLibrary.IsServer`)
              (bind _returnvalue (`SceneComponent.K2_GetComponentToWorld` _array_element))
              (`|SpawnActorFromClass` "/Game/ASSETS/CODE/Turret_Controller/Blueprints/Turret_Projectile_BP.Turret_Projectile_BP_C" _returnvalue "Undefined" "OverrideRootScale" self self)
              (else
                (`self.Spawn Projectile (multicast)` _returnvalue)))))))))

(event `Spawn Projectile (multicast)`
  (params (SpawnTransform :type "Transform Structure"))
  ;[1 1 1] Fire Projectile With Left Click
  ;;[1 1 1] Spawn Projectiles Only If Barrel Is Pointed At Target
  ;;;[1 1 1] Spawn projectile on the server
  (`|SpawnActorFromClass` "/Game/ASSETS/CODE/Turret_Controller/Blueprints/Turret_Projectile_BP.Turret_Projectile_BP_C" SpawnTransform "Undefined" "OverrideRootScale" self self))

(event `Key|RightMouseButton`
  (params (Key :type "Key Structure"))
  ;[1 1 1] Free Camera Rotation
  (:`Pressed`
    (set `self.Free Rotation` true)
    (`/Game/ASSETS/CODE/Turret_Controller/Blueprints/Turret_controller_BP.Free Camera Rotation` (`self.Turret_controller_BP`) (stale _output_get) :!label _label))
  (:`Released`
    (bind _output_get (set `self.Free Rotation` false))
    (goto _label)))

(event `InputAxis|Turn`
  (params (AxisValue :type "Float (single-precision)"))
  ;[1 1 1] Camera Inputs
  (`/Game/ASSETS/CODE/Turret_Controller/Blueprints/Camera_Controller_BP.Add look at direction (Camera)` (`self.Camera_Controller_BP`) AxisValue (stale `InputAxis|LookUp` AxisValue) :!label _label_2))

(event `InputAxis|LookUp`
  (params (AxisValue :type "Float (single-precision)"))
  ;[1 1 1] Camera Inputs
  (goto _label_2))

(fn `UserConstructionScript`)