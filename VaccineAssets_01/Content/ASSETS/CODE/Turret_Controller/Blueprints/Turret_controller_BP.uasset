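; Turret controller component that aims its owner's turrets and barrels at a camera-traced, cached or externally supplied target location.
; BeginPlay finds turret, barrel and emitter components by numbered names, then builds camera and ignore lists.
; Tick rotates each turret within yaw and pitch limits at set speeds, then flags on-target and unobstructed firing lines.
; Server and client events optionally replicate target location and state, throttled by delays.
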(event `self.ReceiveBeginPlay`
  ;[1 1 1] Find turrets components in partent actor and organize them
  (`self.Beginplay Identification Of Turret Components`
    (:`OutputPin`
      ;[1 1 1] Set owner components to variables for easier access
      (`|ExecutionSequence`
        (:`then_0`
          (`self.Create Camera Array`))
        (:`then_1`
          (`self.List Turret Components Debug Option`))
        (:`then_2`
          (`self.Auto Add Actors To Ignore/Not Aim At`))))))

(event `self.ReceiveTick`
  (params (DeltaSeconds :type "Float (single-precision)"))
  ;[1 1 1] Per Tick Events (Rotating Turrets, Finding Target Location, etc...)
  (set `self.Delta seconds` DeltaSeconds)
  (bind _aspawn (cast `Pawn` (`self.GetOwner`))
    (:`then`
      (bind _returnvalue (`Pawn.IsLocallyControlled` _aspawn))
      (set `self.Locally Controlled` _returnvalue)
      (if _returnvalue
        (`|ExecutionSequence` :!label _label
          (:`then_0`
            (if (`self.Is Active`) :!label _label_2
              (`self.Find Target Location`)
              (`self.Rotate Turrets To Face Target Location`)))
          (:`then_1`
            (if (`self.Should Replicate`)
              (`|ExecutionSequence`
                (:`then_0`
                  ;[1 1 1] Update Aim At Location To Other Clients
                  (`KismetSystemLibrary.Delay` 1.0)
                  (set `self.Net Cached Location` (`self.Target Location`))
                  (if (`KismetSystemLibrary.IsServer`)
                    (`/Engine/EditorBlueprintResources/StandardMacros.DoOnce` false :!label _label_3
                      (:`Completed`
                        (`self.Server Update Target Location` (`self.Target Location`))
                        (`KismetSystemLibrary.Delay` (`self.Maximum Update Frequency`) :!label _label_4)
                        (`|ExecutionSequence`
                          (:`then_0`
                            (goto _label_3 :!via `Reset`))
                          (:`then_1`
                            (goto _label_5 :!via `Reset`)))))
                    (else
                      (`self.Client Update Target Location` (`self.Target Location`)))))
                (:`then_1`
                  (if (`KismetSystemLibrary.IsServer`)
                    _
                    (elif (!= (`self.Update Variables Every Nth Seconds`) 0.0)
                      (`KismetSystemLibrary.Delay` (`self.Update Variables Every Nth Seconds`))
                      ;[1 1 1] Update General Variables To Server If Set To.
                      (`self.Client Update Variables` (`self.Is Active`) (`self.Turret Not Active`) (`self.Ignore Actors On Camera Linetrace`) (`self.Targeting Camera`) (`self.Manually provide Target Location`) (`self.Target Location`) (`self.Use Cached Location`) (`self.Turret Array`) (`self.Look At Rotation For Target Location`) (`self.Target Distance`) (`self.Pointed At Freedom`) (`self.Turret Pointed At Target`) (`self.Dont Aim At Actors`) (`self.Unobstructed`)))))))))
        (else
          (goto _label_2))))
    (:`CastFailed`
      (goto _label))))

(event `Client Update Target Location`
  (params (`Target Location` :type "Vector Structure"))
  ;[1 1 1] Update Aim At Location To Other Clients
  (`/Engine/EditorBlueprintResources/StandardMacros.DoOnce` false :!label _label_5
    (:`Completed`
      (`self.Server Update Target Location` `Target Location`)
      (set `self.Target Location` `Target Location`)
      (goto _label_4))))

(event `Client Update Variables`
  (params (`Is Active` :type Boolean) (`Turret Not Active` :type "Array of Boolean") (`Ignore Actors On Camera Linetrace` :type "Array of Actor Object Reference") (`Targeting Camera` :type Integer) (`Manually provide Target Location` :type Boolean) (`Target Location` :type "Vector Structure") (`Use Cached Location` :type Boolean) (`Turret Array` :type "Array of /Game/ASSETS/CODE/Turret_Controller/Blueprints/Turret_variables_Struct Structure") (`Look At Rotation For Target Location` :type "Rotator Structure") (`Target Distance` :type "Array of Float (double-precision)") (`Pointed At Freedom` :type "Float (double-precision)") (`Turret Pointed At Target` :type "Array of Boolean") (`Dont Aim At Actors` :type "Array of Actor Object Reference") (Unobstructed :type "Array of Boolean"))
  ;[1 1 1] Update General Variables To Server If Set To.
  (set `self.Is Active` `Is Active`)
  (set `self.Turret Not Active` `Turret Not Active`)
  (set `self.Ignore Actors On Camera Linetrace` `Ignore Actors On Camera Linetrace`)
  (set `self.Targeting Camera` `Targeting Camera`)
  (set `self.Manually provide Target Location` `Manually provide Target Location`)
  (set `self.Target Location` `Target Location`)
  (set `self.Use Cached Location` `Use Cached Location`)
  (set `self.Turret Array` `Turret Array`)
  (set `self.Look At Rotation For Target Location` `Look At Rotation For Target Location`)
  (set `self.Target Distance` `Target Distance`)
  (set `self.Pointed At Freedom` `Pointed At Freedom`)
  (set `self.Turret Pointed At Target` `Turret Pointed At Target`))

(event `Free Camera Rotation`
  (params (Enabled :type Boolean))
  ;[1 1 1] Free Camera Rotation (When Enabled The Turret Continues Rotating/Resting At The Last Target Location, Allowing Camera Movement Without Altering Turrets Target Direction.
  (set `self.Use Cached Location` Enabled))

(event `Server Update Is Active`
  (params (`Is Active` :type Boolean))
  ;[1 1 1] Recieve Remote Turret Control BPI messages.
  (set `self.Is Active` `Is Active`))

(event `/Game/ASSETS/CODE/Turret_Controller/Blueprints/Remote_Turret_Control_BPI.Turret Enable`
  (params (`Turret Enabled` :type Boolean))
  ;[1 1 1] Recieve Remote Turret Control BPI messages.
  (bind _output_get (set `self.Is Active` `Turret Enabled`))
  (`self.Server Update Is Active` _output_get))

(event `Server Update Override Camera`
  (params (`Override Camera` :type "SceneComponent Object Reference"))
  ;[1 1 1] Recieve Remote Turret Control BPI messages.
  (set `self.Override Camera` `Override Camera`))

(event `/Game/ASSETS/CODE/Turret_Controller/Blueprints/Remote_Turret_Control_BPI.Set Turret Override Camera`
  (params (`Override Camera` :type "SceneComponent Object Reference"))
  ;[1 1 1] Recieve Remote Turret Control BPI messages.
  (bind _output_get (set `self.Override Camera` `Override Camera`))
  (`self.Server Update Override Camera` _output_get))

(event `/Game/ASSETS/CODE/Turret_Controller/Blueprints/Remote_Turret_Control_BPI.Turret Target Location`
  (params (`Aim At Location` :type "Vector Structure"))
  ;[1 1 1] Recieve Remote Turret Control BPI messages.
  (bind _output_get (set `self.Target Location` `Aim At Location`))
  (`self.Server Update Target Location` _output_get))

(event `Server Update Target Location`
  (params (`Target Location` :type "Vector Structure"))
  ;[1 1 1] Recieve Remote Turret Control BPI messages.
  (if (not (`self.Locally Controlled`))
    (set `self.Target Location` `Target Location`)
    (set `self.Target Location Recieved` true)))

(event `/Game/ASSETS/CODE/Turret_Controller/Blueprints/Remote_Turret_Control_BPI.Update Turret Rotation Limits`
  (params (Left :type "Float (single-precision)") (Right :type "Float (single-precision)") (Up :type "Float (single-precision)") (Down :type "Float (single-precision)") (`Limit Horizontal` :type Boolean) (`Limit Vertical` :type Boolean) (`Turret Index` :type Integer))
  (bind (_output_turret _output_barrel _output_projectileemitter _output_limitturretrotation _output_limitbarrelrotation _output_rotateturretleftlimit _output_rotateturretrightlimit _output_rotatebarreluplimit _output_rotatebarreldownlimit) (break `/Game/ASSETS/CODE/Turret_Controller/Blueprints/Turret_variables_Struct` (`|GetArrayItem` (`self.Turret Array`) `Turret Index`)))
  ;[1 1 1] Recieve Remote Turret Control BPI messages.
  (`|VariableSetRef` _output_limitturretrotation `Limit Horizontal`)
  (`|VariableSetRef` _output_limitbarrelrotation `Limit Vertical`)
  (`|VariableSetRef` _output_rotateturretleftlimit Left)
  (`|VariableSetRef` _output_rotateturretrightlimit Right)
  (`|VariableSetRef` _output_rotatebarreluplimit Up)
  (`|VariableSetRef` _output_rotatebarreldownlimit Down)
  (if (`KismetSystemLibrary.IsServer`)
    (`self.Server Update Turret Array` (`self.Turret Array`))))

(event `Server Update Turret Array`
  (params (`Turret Array` :type "Array of /Game/ASSETS/CODE/Turret_Controller/Blueprints/Turret_variables_Struct Structure"))
  ;[1 1 1] Recieve Remote Turret Control BPI messages.
  (set `self.Turret Array` `Turret Array`))

(fn `Restricted Aiming`
  (params (`Current Rotation` :type "Float (double-precision)") (`Target Rotation` :type "Float (double-precision)") (`Posotive Limit` :type "Float (double-precision)") (`Negative Limit` :type "Float (double-precision)") (`Rotation Rate` :type "Float (double-precision)") (`Rotation Limited` :type Boolean) (`Delta Seconds` :type "Float (double-precision)"))
  (returns (`Output Rotaiton` :type "Float (double-precision)"))
  (locals (`Output Rotation` :type "Float (double-precision)" :default 0.0) (D_Seconds :type "Float (double-precision)") (`Input Rotation Rate` :type "Float (double-precision)") (`Input Current Rotation` :type "Float (double-precision)") (`Input Target Rotation` :type "Float (double-precision)") (`Input Posotive Limit` :type "Float (double-precision)") (`Input Negative Limit` :type "Float (double-precision)"))
  (bind _input_negative_limit (`local.Input Negative Limit`))
  (bind _input_target_rotation (`local.Input Target Rotation`))
  (bind _returnvalue (+ (`local.Input Posotive Limit`) _input_negative_limit))
  (bind _returnvalue_2 (/ _returnvalue 2.0))
  (bind _returnvalue_3 (- _returnvalue _returnvalue_2))
  ;[1 1 1] Set Variables On Start
  (set `local.Input Current Rotation` `Current Rotation`)
  (set `local.Input Target Rotation` `Target Rotation`)
  (set `local.Input Posotive Limit` `Posotive Limit`)
  (set `local.Input Negative Limit` `Negative Limit`)
  (set `local.Input Rotation Rate` `Rotation Rate`)
  (set `local.D_Seconds` `Delta Seconds`)
  (if `Rotation Limited`
    ;[1 1 1] Interp the float in the direction that lets it get closest to the new target value after taking limits into account
    (if (or (`KismetMathLibrary.InRange_FloatFloat` _input_target_rotation _returnvalue_2 (+ _returnvalue_3 (`local.Input Posotive Limit`))) (`KismetMathLibrary.InRange_FloatFloat` _input_target_rotation (- (* _input_negative_limit -1.0) _returnvalue_3) _returnvalue_2))
      ;[1 1 1] Make Sure Output Rotation Is Within Limits
      (set `local.Output Rotation` (`KismetMathLibrary.FClamp` (`KismetMathLibrary.FInterpTo_Constant` (`local.Input Current Rotation`) (`local.Input Target Rotation`) (`local.D_Seconds`) (`local.Input Rotation Rate`)) (* (`local.Input Negative Limit`) -1.0) (`local.Input Posotive Limit`)))
      (return (stale _output_get)))
    (else
      ;[1 1 1] Interp Value Directly Towards Target Value
      (bind _output_get (set `local.Output Rotation` (.roll (`KismetMathLibrary.RInterpTo_Constant` (`KismetMathLibrary.MakeRotator` (`local.Input Current Rotation`)) (`KismetMathLibrary.MakeRotator` (`local.Input Target Rotation`)) (`local.D_Seconds`) (`local.Input Rotation Rate`)))))
      (return _output_get))))