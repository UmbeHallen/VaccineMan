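; Player vehicle character Blueprint: a drivable, drifting vehicle with a turret that fires projectiles.
; Input feeds throttle, steering and drift to MovementComponent, look to CameraControllerBP, and right-mouse free rotation to TurretControllerBP.
; Holding left mouse runs a timeline, rate-scaled by FireRate, whose event spawns projectiles at Emitter1.
; BeginPlay adds the HUD crosshair and Info_To_UI exposes stats; the Q/E GunMode switch only feeds disconnected logic.
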(event `self.ReceiveBeginPlay`
  ;[1 1 1] BEGIN PLAY
  (bind _vaccincontroller_ref (message `/Game/GAME_FOLDER/CORE/UTILITY/InterfaceEnumsStructs/BPI_Main_Interface.GetPlayerControllerReference` (`GameplayStatics.GetPlayerController` 0)))
  (set `self.Vaccin Controller Ref` _vaccincontroller_ref)
  (`self.UI_SetUP_BeginPlay`)
  (`self.Fire Rate Set Up Begin Play`))

(event `UI_SetUP_BeginPlay`
  ;[1 1 1] UI SETUP / From begin play
  (`/Game/ASSETS/UI/ProHUDV2/Blueprints/Libraries/BPi_HUDManagerV2.AddCrosshair` :`self` (`/Game/ASSETS/UI/ProHUDV2/Blueprints/Libraries/BP_PHV2_Functions.GetHUDManager`)))

(event `Fire Rate Set Up Begin Play`
  ;[1 1 1] Setting up FireRate
  (`TimelineComponent.SetPlayRate` (`self.RapidFire_TimeLine`) (/ 1.0 (`self.FireRate`))))

(event `Key|RightMouseButton`
  (params (Key :type "Key Structure"))
  ;[1 1 1] Free Camera Rotation
  (:`Pressed`
    (set `self.Free Rotation` true)
    (`/Game/ASSETS/CODE/Turret_Controller/Blueprints/Turret_controller_BP.Free Camera Rotation` (`self.Turret_controller_BP`) (stale _output_get) :!label _label))
  (:`Released`
    (bind _output_get (set `self.Free Rotation` false))
    (goto _label)))

(event `InputAxis|MoveForward`
  (params (AxisValue :type "Float (single-precision)"))
  ;[1 1 1] Basic inputs for the vehicle.
  (bind _output_get (set `self.MoveForward` AxisValue))
  (`ArcadeVehicleMovementComponentBase.SetAccelerationInput` (`self.MovementComponent`) _output_get))

(event `InputAxis|MoveRight`
  (params (AxisValue :type "Float (single-precision)"))
  ;[1 1 1] Basic inputs for the vehicle.
  (bind _output_get (set `self.MoveRightAxsisValue` AxisValue))
  (`ArcadeVehicleMovementComponentBase.SetTurningInput` (`self.MovementComponent`) _output_get))

(event `InputAction|Drift`
  (params (Key :type "Key Structure"))
  (bind _movementcomponent (`self.MovementComponent`))
  ;[1 1 1] Basic inputs for the vehicle.
  (:`Pressed`
    (`ArcadeVehicleMovementComponentBase.SetDriftInput` _movementcomponent true))
  (:`Released`
    (`ArcadeVehicleMovementComponentBase.SetDriftInput` _movementcomponent false)))

(event `InputAxis|Turn`
  (params (AxisValue :type "Float (single-precision)"))
  ;[1 1 1] Basic inputs for the vehicle.
  (`/Game/ASSETS/CODE/Turret_Controller/Blueprints/Camera_Controller_BP.Add look at direction (Camera)` (`self.Camera_Controller_BP`) AxisValue (stale `InputAxis|LookUp` AxisValue) :!label _label_2))

(event `InputAxis|LookUp`
  (params (AxisValue :type "Float (single-precision)"))
  ;[1 1 1] Basic inputs for the vehicle.
  (goto _label_2))

(event `Key|Q`
  (params (Key :type "Key Structure"))
  ;[1 1 1] Dev Logic switching gune use
  (:`Pressed`
    (set `self.GunMode` true)))

(event `Key|E`
  (params (Key :type "Key Structure"))
  ;[1 1 1] Dev Logic switching gune use
  (:`Pressed`
    (set `self.GunMode` false)))

(event `Key|LeftMouseButton`
  (params (Key :type "Key Structure"))
  (bind (_returnvalue_location _returnvalue_rotation) (`KismetMathLibrary.BreakTransform` (`SceneComponent.K2_GetComponentToWorld` (`self.Emitter1`))))
  ;[0 0 0] FireLogic
  (:`Pressed`
    (`Timeline|RapidFire_TimeLine` :!via `PlayFromStart` :!label _label_3
      (:`FIRE!`
        (`|MultiGate` false true
          (:`Out 0`
            ;[0 0 0] FireLogic
            (`|SpawnActorFromClass` "/Game/GAME_FOLDER/CORE/BLUEPRINTS/PROJECTILES/BP_PlayerProjectileBase1.BP_PlayerProjectileBase1_C" (`KismetMathLibrary.MakeTransform` _returnvalue_location _returnvalue_rotation (2.0 2.0 2.0)) "Undefined" "OverrideRootScale" self self))))))
  (:`Released`
    (goto _label_3 :!via `Stop`)))

(fn `GetPlayerControllerReference`
  (returns (VaccinController_ref :type "/Game/GAME_FOLDER/CORE/CHARACTER/BP_VaccinController Object Reference"))
  (return null))

(fn `Info_To_UI`
  (returns (Speed_level :type Integer) (Resistance_Level :type Integer) (Dmg_level :type Integer) (Curretn_Resistance :type Integer) (CurrentBodyHealth :type "Float (double-precision)") (AgeInminutes :type Integer))
  (return (`self.Speed Level`) (`self.Resistance Level`) (`self.Dmg Level`) (`self.Curretn Resistance`) 0.0 0))

(fn `ObjectiveGeneralCall`
  (returns (ObjectiveType :type "/Game/GAME_FOLDER/CORE/UTILITY/InterfaceEnumsStructs/E_ObjectiveType Enum") (ObjectiveSeverity :type "Float (double-precision)"))
  (return "NewEnumerator0" 0.0))

(fn `UserConstructionScript`
  (`parent.UserConstructionScript`))