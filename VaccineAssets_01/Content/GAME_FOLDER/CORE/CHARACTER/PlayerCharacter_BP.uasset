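; Player-controlled vehicle with a turret that sets up the crosshair and main gameplay HUD on BeginPlay.
; Movement axes and drift feed MovementComponent, while look axes drive CameraControllerBP and right mouse toggles free camera rotation on TurretControllerBP.
; Holding left mouse runs a timeline that spawns a turret projectile at Emitter1 on every update with shooting VFX.
; Info_To_UI returns only zeroed stats.
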(event `self.ReceiveBeginPlay`
  ;[1 1 1] BEGIN PLAY
  (`self.UI_SetUP_BeginPlay`))

(event `UI_SetUP_BeginPlay`
  ;[1 1 1] UI SETUP / From begin play
  (`/Game/ASSETS/UI/ProHUDV2/Blueprints/Libraries/BPi_HUDManagerV2.AddCrosshair` :`self` (`/Game/ASSETS/UI/ProHUDV2/Blueprints/Libraries/BP_PHV2_Functions.GetHUDManager`))
  ;[1 1 1] UI SETUP / From begin play / Main GameplayHUD
  (bind _returnvalue (`|CreateWidget` (`self.MainGamePlay_Hud`)))
  (`UserWidget.AddToViewport` _returnvalue 0))

(event `Key|RightMouseButton`
  (params (Key :type "Key Structure"))
  ;[1 1 1] Free Camera Rotation
  (:`Pressed`
    (set `self.Free Rotation` true)
    (`/Game/ASSETS/CODE/Turret_Controller/Blueprints/Turret_controller_BP.Free Camera Rotation` (`self.Turret_controller_BP`) (stale _output_get) :!label _label))
  (:`Released`
    (bind _output_get (set `self.Free Rotation` false))
    (goto _label)))

(event `InputAxis|MoveForward`
  (params (AxisValue :type "Float (single-precision)"))
  ;[1 1 1] Basic inputs for the vehicle.
  (bind _output_get (set `self.MoveForward` AxisValue))
  (`ArcadeVehicleMovementComponentBase.SetAccelerationInput` (`self.MovementComponent`) _output_get))

(event `InputAxis|MoveRight`
  (params (AxisValue :type "Float (single-precision)"))
  ;[1 1 1] Basic inputs for the vehicle.
  (bind _output_get (set `self.MoveRightAxsisValue` AxisValue))
  (`ArcadeVehicleMovementComponentBase.SetTurningInput` (`self.MovementComponent`) _output_get))

(event `InputAction|Drift`
  (params (Key :type "Key Structure"))
  (bind _movementcomponent (`self.MovementComponent`))
  ;[1 1 1] Basic inputs for the vehicle.
  (:`Pressed`
    (`ArcadeVehicleMovementComponentBase.SetDriftInput` _movementcomponent true))
  (:`Released`
    (`ArcadeVehicleMovementComponentBase.SetDriftInput` _movementcomponent false)))

(event `InputAxis|Turn`
  (params (AxisValue :type "Float (single-precision)"))
  ;[1 1 1] Basic inputs for the vehicle.
  (`/Game/ASSETS/CODE/Turret_Controller/Blueprints/Camera_Controller_BP.Add look at direction (Camera)` (`self.Camera_Controller_BP`) AxisValue (stale `InputAxis|LookUp` AxisValue) :!label _label_2))

(event `InputAxis|LookUp`
  (params (AxisValue :type "Float (single-precision)"))
  ;[1 1 1] Basic inputs for the vehicle.
  (goto _label_2))

(event `Key|LeftMouseButton`
  (params (Key :type "Key Structure"))
  (bind (_returnvalue_location _returnvalue_rotation) (`KismetMathLibrary.BreakTransform` (`SceneComponent.K2_GetComponentToWorld` (`self.Emitter1`))))
  ;[1 1 1] FireLogic
  (:`Pressed`
    (`|ExecutionSequence`
      (:`then_0`
        (`|MultiGate` false true))
      (:`then_1`
        (`Timeline|Timeline_0` :!via `PlayFromStart` :!label _label_3
          (:`Update`
            (`|SpawnActorFromClass` "/Game/ASSETS/CODE/Turret_Controller/Blueprints/Turret_Projectile_BP.Turret_Projectile_BP_C" (`KismetMathLibrary.MakeTransform` _returnvalue_location _returnvalue_rotation (2.0 2.0 2.0)) "Undefined" "OverrideRootScale" self self)
            (`ActorComponent.Activate` (`self.Shooting_Vfx`) false))))))
  (:`Released`
    (`|ExecutionSequence`
      (:`then_0`
        (goto _label_3 :!via `Stop`))
      (:`then_1`
        (`ActorComponent.Deactivate` (`self.Shooting_Vfx`))))))

(fn `Info_To_UI`
  (returns (Speed_level :type Integer) (Resistance_Level :type Integer) (Dmg_level :type Integer) (Curretn_Resistance :type Integer))
  (return 0 0 0 0))

(fn `UserConstructionScript`
  (`parent.UserConstructionScript`))