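; BP_VaccinController is a controller for the vaccine character that tracks its resistance and upgrade levels.
; Incoming damage lowers current resistance by one and asks the HUD manager for a red damage effect.
; Upgrade events increment resistance and damage levels, while the speed upgrade and zero-resistance death check are empty stubs.
; Getters expose the controller itself and UI stats, though the stats function returns only zeros rather than the tracked values.
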(event `/Game/GAME_FOLDER/CORE/UTILITY/InterfaceEnumsStructs/BPI_Main_Interface.To_VaccinController`
  (params (DMG :type "/Game/GAME_FOLDER/CORE/UTILITY/InterfaceEnumsStructs/E_To_Player_infoType Enum" :default "NewEnumerator0"))
  (switch `/Game/GAME_FOLDER/CORE/UTILITY/InterfaceEnumsStructs/E_To_Player_infoType` DMG
    (:`NewEnumerator0`
      (set `self.Curretn Resistance` (- (`self.Curretn Resistance`) 1))
      (`/Game/ASSETS/UI/ProHUDV2/Blueprints/Libraries/BPi_HUDManagerV2.CreateHUDFX_Damage` (`/Game/ASSETS/UI/ProHUDV2/Blueprints/Libraries/BP_PHV2_Functions.GetHUDManager`) (struct :`R` 1.0 :`A` 0.25) (struct :`R` 0.614583 :`A` 0.374) false (0.0 1.0) 0.2 0.4))))

(event `Event_Uppgrade_Resistance`
  ;[1 0.4936 0 1 14] CustomEvent [ ADD RESISTANCE ]
  (set `self.Resistance Level` (+ (`self.Resistance Level`) 1)))

(event `Uppgrade_Speed`
  ;[1 0.4936 0 1 14] CustomEvent [ UPPGRADE SPEED ]
)

(event `DeathCheck`
  ;[0 0 0] CustomEvent [ Take DMG ]
  (if (== (`self.Curretn Resistance`) 0)
    _))

(event `Event_Uppgrade_DMG`
  ;[1 0.4936 0] CustomEvent [ UPPGRADE DMG ]
  (set `self.Dmg Level` (+ (`self.Dmg Level`) 1)))

(fn `GetPlayerControllerReference`
  (returns (VaccinController_ref :type "/Game/GAME_FOLDER/CORE/CHARACTER/BP_VaccinController Object Reference"))
  (return self))

(fn `Info_To_UI`
  (returns (Speed_level :type Integer) (Resistance_Level :type Integer) (Dmg_level :type Integer) (Curretn_Resistance :type Integer))
  (return 0 0 0 0))

(fn `UserConstructionScript`)