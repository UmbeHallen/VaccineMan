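; Player hover bike child Blueprint that adds mouse-driven projectile shooting.
; Holding left mouse plays a timeline whose fire event spawns projectiles and triggers shooting VFX, using looping MultiGates to alternate emitters.
; GunMode selects between two emitters and four, each set with its own projectile class.
; BeginPlay is empty, leaving the controller reference, crosshair/HUD and fire-rate timeline setup unwired.
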(event `self.ReceiveBeginPlay`
  ;[1 1 1] BEGIN PLAY
)

(event `UI_SetUP_BeginPlay`
  ;[1 1 1] UI SETUP / From begin play
  (`/Game/ASSETS/UI/ProHUDV2/Blueprints/Libraries/BPi_HUDManagerV2.AddCrosshair` :`self` (`/Game/ASSETS/UI/ProHUDV2/Blueprints/Libraries/BP_PHV2_Functions.GetHUDManager`))
  ;[1 1 1] UI SETUP / From begin play / Main GameplayHUD
  (bind _returnvalue (`|CreateWidget` (`self.MainGamePlay_Hud`)))
  (`UserWidget.AddToViewport` _returnvalue 0))

(event `Fire Rate Set Up Begin Play`
  ;[1 1 1] Setting up FireRate
  (`TimelineComponent.SetPlayRate` (`self.FireTimeLine`) (/ 1.0 (`self.FireRate`))))

(event `Key|LeftMouseButton`
  (params (Key :type "Key Structure"))
  (bind (_returnvalue_location _returnvalue_rotation) (`KismetMathLibrary.BreakTransform` (`SceneComponent.K2_GetComponentToWorld` (`self.Emitter3`))))
  (bind (_returnvalue_location_2 _returnvalue_rotation_2) (`KismetMathLibrary.BreakTransform` (`SceneComponent.K2_GetComponentToWorld` (`self.Emitter1`))))
  (bind (_returnvalue_location_3 _returnvalue_rotation_3) (`KismetMathLibrary.BreakTransform` (`SceneComponent.K2_GetComponentToWorld` (`self.Emitter2`))))
  (bind (_returnvalue_location_4 _returnvalue_rotation_4) (`KismetMathLibrary.BreakTransform` (`SceneComponent.K2_GetComponentToWorld` (`self.Emitter4`))))
  (bind (_returnvalue_location_5 _returnvalue_rotation_5) (`KismetMathLibrary.BreakTransform` (`SceneComponent.K2_GetComponentToWorld` (`self.Emitter5`))))
  (bind (_returnvalue_location_6 _returnvalue_rotation_6) (`KismetMathLibrary.BreakTransform` (`SceneComponent.K2_GetComponentToWorld` (`self.Emitter6`))))
  ;[0 0 0] FireLogic
  (:`Pressed`
    (`Timeline|FireTimeLine` :!via `PlayFromStart` :!label _label
      (:`FIRE!`
        (if (`self.GunMode`)
          (`|MultiGate` false true
            (:`Out 0`
              ;[0 0 0] FireLogic
              (`|SpawnActorFromClass` "/Game/GAME_FOLDER/CORE/BLUEPRINTS/PROJECTILES/BP_PlayerProjectileBase1.BP_PlayerProjectileBase1_C" (`KismetMathLibrary.MakeTransform` _returnvalue_location_2 _returnvalue_rotation_2 (2.0 2.0 2.0)) "Undefined" "OverrideRootScale" self self)
              (`ActorComponent.Activate` (`self.Shooting_Vfx`) false))
            (:`Out 1`
              (`|SpawnActorFromClass` "/Game/GAME_FOLDER/CORE/BLUEPRINTS/PROJECTILES/BP_PlayerProjectileBase1.BP_PlayerProjectileBase1_C" (`KismetMathLibrary.MakeTransform` _returnvalue_location_3 _returnvalue_rotation_3 (2.0 2.0 2.0)) "Undefined" "OverrideRootScale" self self)
              (`ActorComponent.Activate` (`self.Shooting_Vfx`) false)))
          (else
            (`|MultiGate` false true
              (:`Out 0`
                ;[0 0 0] FireLogic
                (`|SpawnActorFromClass` "/Game/GAME_FOLDER/CORE/BLUEPRINTS/PROJECTILES/BP_PlayerProjectileBase.BP_PlayerProjectileBase_C" (`KismetMathLibrary.MakeTransform` _returnvalue_location_5 _returnvalue_rotation_5 (2.0 2.0 2.0)) "Undefined" "OverrideRootScale" self self)
                (`ActorComponent.Activate` (`self.Shooting_Vfx`) false))
              (:`Out 1`
                (`|SpawnActorFromClass` "/Game/GAME_FOLDER/CORE/BLUEPRINTS/PROJECTILES/BP_PlayerProjectileBase.BP_PlayerProjectileBase_C" (`KismetMathLibrary.MakeTransform` _returnvalue_location_6 _returnvalue_rotation_6 (2.0 2.0 2.0)) "Undefined" "OverrideRootScale" self self)
                (`ActorComponent.Activate` (`self.Shooting_Vfx`) false))
              (:`Out 2`
                (`|SpawnActorFromClass` "/Game/GAME_FOLDER/CORE/BLUEPRINTS/PROJECTILES/BP_PlayerProjectileBase.BP_PlayerProjectileBase_C" (`KismetMathLibrary.MakeTransform` _returnvalue_location _returnvalue_rotation (2.0 2.0 2.0)) "Undefined" "OverrideRootScale" self self)
                (`ActorComponent.Activate` (`self.Shooting_Vfx`) false))
              (:`Out 3`
                (`|SpawnActorFromClass` "/Game/GAME_FOLDER/CORE/BLUEPRINTS/PROJECTILES/BP_PlayerProjectileBase.BP_PlayerProjectileBase_C" (`KismetMathLibrary.MakeTransform` _returnvalue_location_4 _returnvalue_rotation_4 (2.0 2.0 2.0)) "Undefined" "OverrideRootScale" self self)
                (`ActorComponent.Activate` (`self.Shooting_Vfx`) false))))))))
  (:`Released`
    (goto _label :!via `Stop`)))

(fn `UserConstructionScript`
  (`parent.UserConstructionScript`))