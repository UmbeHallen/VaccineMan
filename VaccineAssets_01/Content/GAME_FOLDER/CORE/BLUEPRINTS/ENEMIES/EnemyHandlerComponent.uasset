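; Enemy handler component that stores an enemy's health, weakness and strength and processes incoming hits.
; Hit triggers HUD hit feedback, doubles or halves damage by type match, triples crits, and spawns damage text at impact.
; Weakness, strength and default hits share one text style; only crits differ.
; The health step sets Health to damage minus Health, apparently reversed, and its zero-health branch is empty.
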(event `Set Enemy Inital Values`
  (params (Weakness :type "/Game/GAME_FOLDER/CORE/UTILITY/InterfaceEnumsStructs/E_DmgType Enum" :default "NewEnumerator0") (Strenghts :type "/Game/GAME_FOLDER/CORE/UTILITY/InterfaceEnumsStructs/E_DmgType Enum" :default "NewEnumerator0") (Health :type "Float (double-precision)"))
  ;[0 0 0] Sets inital values for the Enemy Actor
  (set `self.Weakness` Weakness)
  (set `self.Strenghts` Strenghts)
  (set `self.Health` Health))

(event `Hit`
  (params (DmgType :type "/Game/GAME_FOLDER/CORE/UTILITY/InterfaceEnumsStructs/E_DmgType Enum" :default "NewEnumerator0") (IncomingDMG :type "Float (double-precision)") (`Crit?` :type Boolean) (ImpactLocation :type "Vector Structure"))
  (set `self.Impact Location` ImpactLocation)
  ;[0 0 0] Store latest Incoming Data
  (set `self.Incoming [Dmg Type}` DmgType)
  (set `self.Incoming [DMG]` IncomingDMG)
  (set `self.incoming [Crit?}` `Crit?`)
  ;[0 0 0] Creat Hit marker effect
  (`/Game/ASSETS/UI/ProHUDV2/Blueprints/Libraries/BPi_HUDManagerV2.HitFeedback` (`/Game/ASSETS/UI/ProHUDV2/Blueprints/Libraries/BP_PHV2_Functions.GetHUDManager`) 0.125 (struct :`R` 0.833333 :`G` 0.802035 :`B` 0.831408 :`A` 0.88) "NewEnumerator1" (struct :`R` 1.0 :`G` 0.018907 :`A` 1.0) 8.0 1.0)
  ;[0 0 0 1 12] Check if Hit came from Type same as this Enemys weakness
  (if (`|EnumEquality` (`self.Incoming [Dmg Type}`) (`self.Weakness`))
    ;[0 0 0 1 15] Set New Value
    (set `self.Incoming [DMG]` (`KismetMathLibrary.FClamp` (* (`self.Incoming [DMG]`) 2.0) 1.0 1000000000.0))
    ;[0 0 0 1 15] Setting [ WEAKNESS ] Visuals on text effect
    (set `self.E Damage Text type` "NewEnumerator0")
    (else
      ;[0 0 0 1 12] Check if Hit came from Type same as this Enemys Streght
      (if (`|EnumEquality` (`self.Incoming [Dmg Type}`) (`self.Strenghts`))
        ;[0 0 0 1 15] Set New Value
        (set `self.Incoming [DMG]` (`KismetMathLibrary.FClamp` (/ (`self.Incoming [DMG]`) 2.0) 1.0 1000000000.0))
        ;[0 0 0 1 15] Setting [ STRENGHT ] Visuals on text effect
        (set `self.E Damage Text type` "NewEnumerator0")
        (else
          ;[0 0 0 1 15] Setting [ DEFAULT ] Visuals on text effect
          (set `self.E Damage Text type` "NewEnumerator0")))))
  (set `self.ParentActorLocation` (`self.Impact Location`))
  ;[0 0 0 1 15] Check if Hit was critical
  ; This code runs on the projectile
  (if (`self.incoming [Crit?}`)
    ;[0 0 0 1 15] Apply Crit multiply
    (set `self.FinalValue [Calculated]` (`KismetMathLibrary.FClamp` (* (`self.Incoming [DMG]`) 3.0) 1.0 1000000000.0))
    ;[0 0 0 1 15] Setting [ CRIT ] Visuals on text effect
    (set `self.E Damage Text type` "NewEnumerator1")
    (else
      ;[0 0 0 1 15] No Value Change
      (set `self.FinalValue [Calculated]` (`self.Incoming [DMG]`))))
  ;[0 1 0.02155] FIRE EFFECT
  (`/Game/ASSETS/CODE/DamageText/Blueprints/BP_DTMacroLibraryOnComponent.CreateDamageText` (`self.ParentActorLocation`) (`KismetTextLibrary.Conv_Int64ToText` (`KismetMathLibrary.FCeil64` (`self.FinalValue [Calculated]`))) (`self.E Damage Text type`))
  ;[0 0.4675 1] Runs the health check and change [ On this blueprint ]
  (`self.InitiateHealthCaluclation` (`self.FinalValue [Calculated]`)))

(event `InitiateHealthCaluclation`
  (params (`IncomingDmg [Caluclated]` :type "Float (double-precision)"))
  (set `self.Health` (- `IncomingDmg [Caluclated]` (`self.Health`)))
  (if (>= 0.0 (`self.Health`))
    _))