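; Base enemy pod turret that aims at and shoots projectiles at the player inside its fire range sphere.
; Range overlap starts a looping fire timer and a timeline scaling bubble, shield and core from zero; leaving clears the timer.
; Tick turns the aim base toward the target, and construction sizes the sphere from pod data.
; Hits pass random test crit damage to EnemyHandlerComponent; the bubble and slime hit-effect chains are disconnected.
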(event `self.ReceiveBeginPlay`
  ;[0 0 0] EVENT BEGINPLAY
  (`self.DecreaseHealth` -10.0)
  (`self.SetScaleValues`))

(event `self.ReceiveTick`
  (params (DeltaSeconds :type "Float (single-precision)"))
  ;[0 0 0] EVENT TICK
  (`self.LookAtUpdate`))

(event `self.FireRange.OnComponentBeginOverlap`
  (params (OverlappedComponent :type "PrimitiveComponent Object Reference") (OtherActor :type "Actor Object Reference") (OtherComp :type "PrimitiveComponent Object Reference") (OtherBodyIndex :type Integer) (bFromSweep :type Boolean) (SweepResult :type "HitResult Structure (by ref)"))
  (bind _returnvalue (`GameplayStatics.GetPlayerPawn` 0))
  ;[1 0.1 0.1] Detect target unity and save reference variable
  (if (== OtherActor _returnvalue)
    (set `self.Target ref` _returnvalue)
    (set `self.HasTarget` true)
    ;[1 0.1 0.1] Shoot handler and Fire Rate
    (bind _returnvalue_2 (`KismetSystemLibrary.K2_SetTimerDelegate` (delegate `Shoot`) 0.4 true))
    (if (`self.HasTarget`)
      (set `self.FireEventHandler` _returnvalue_2)
      (`self.GrowFully`)
      (else
        (`KismetSystemLibrary.K2_ClearAndInvalidateTimerHandle` (`self.FireEventHandler`))))))

(event `Shoot`
  (bind (_returnvalue_location _returnvalue_rotation) (`KismetMathLibrary.BreakTransform` (`SceneComponent.K2_GetComponentToWorld` (`self.Arrow`))))
  ;[1 0.1 0.1] Shoot handler and Fire Rate
  ;[1 0.1 0.1] Shoot Action
  (`|SpawnActorFromClass` "/Game/GAME_FOLDER/CORE/BLUEPRINTS/PROJECTILES/BP_EnemyProjectileBase.BP_EnemyProjectileBase_C" (`KismetMathLibrary.MakeTransform` _returnvalue_location _returnvalue_rotation (3.0 3.0 3.0)) "Undefined" "OverrideRootScale" null null))

(event `self.FireRange.OnComponentEndOverlap`
  (params (OverlappedComponent :type "PrimitiveComponent Object Reference") (OtherActor :type "Actor Object Reference") (OtherComp :type "PrimitiveComponent Object Reference") (OtherBodyIndex :type Integer))
  (bind _returnvalue (`GameplayStatics.GetPlayerPawn` 0))
  ;[1 0.1 0.1] Clear or set new target
  (if (== OtherActor _returnvalue)
    (set `self.HasTarget` false)
    (set `self.Target ref` _returnvalue)
    ;[1 0.1 0.1] Clear shoot timer
    (`KismetSystemLibrary.K2_ClearAndInvalidateTimerHandle` (`self.FireEventHandler`))))

(event `LookAtUpdate`
  (bind (_returnvalue_roll _returnvalue_pitch _returnvalue_yaw) (`KismetMathLibrary.BreakRotator` (`KismetMathLibrary.FindLookAtRotation` (`SceneComponent.K2_GetComponentLocation` (`self.AimBaseComponent`)) (`SceneComponent.K2_GetComponentLocation` (`Actor.RootComponent` (`self.Target ref`))))))
  ;[0 0 0] Look at target
  (if (`self.HasTarget`)
    (`SceneComponent.K2_SetWorldRotation` (`self.AimBaseComponent`) (`KismetMathLibrary.MakeRotator` 0.0 _returnvalue_pitch _returnvalue_yaw) false false)))

(event `SetScaleValues`
  ;[1 1 1] Set Scale Values
  (set `self.ParticleBubbleScale` (`SceneComponent.RelativeScale3D` (`self.NPS_WaterBubble`)))
  (set `self.MeshBubbleScale` (`SceneComponent.RelativeScale3D` (`self.SM_WaterBubble`)))
  (set `self.ParticleSlimeScale` (`SceneComponent.RelativeScale3D` (`self.NPS_SlimeShield`)))
  (set `self.CoreScale` (`SceneComponent.RelativeScale3D` (`self.Core`))))

(event `GrowFully`
  ;[1 1 1] Update Scale at spawn
  (`PrimitiveComponent.CreateDynamicMaterialInstance` (`self.SM_WaterBubble`) 0 "/Game/ASSETS/VFX/Shield_FX_Niagara/Niagara_Shield/Material/M_waterDrop1_Inst3.M_waterDrop1_Inst3" "None")
  (set `self.IsFullyGrown?` true)
  (bind (_direction _percentage) (`Timeline|GrowthCycle` :!label _label)
    (:`Update`
      (`SceneComponent.K2_SetRelativeTransform` (`self.NPS_WaterBubble`) (`KismetMathLibrary.MakeTransform` (0.0 0.0 0.0) (struct) (`KismetMathLibrary.VLerp` (0.0 0.0 0.0) (`self.ParticleBubbleScale`) _percentage)) false false)
      (`SceneComponent.K2_SetRelativeTransform` (`self.SM_WaterBubble`) (`KismetMathLibrary.MakeTransform` (0.0 0.0 0.0) (struct) (`KismetMathLibrary.VLerp` (0.0 0.0 0.0) (`self.MeshBubbleScale`) _percentage)) false false)
      (`SceneComponent.K2_SetRelativeTransform` (`self.NPS_SlimeShield`) (`KismetMathLibrary.MakeTransform` (0.0 0.0 0.0) (struct) (`KismetMathLibrary.VLerp` (0.0 0.0 0.0) (`self.ParticleSlimeScale`) _percentage)) false false)
      (`SceneComponent.K2_SetRelativeTransform` (`self.Core`) (`KismetMathLibrary.MakeTransform` (0.0 0.0 0.0) (struct) (`KismetMathLibrary.VLerp` (0.0 0.0 0.0) (`self.CoreScale`) _percentage)) false false))
    (:`StopGrowth`
      (if (not (`self.IsFullyGrown?`))
        (`self.GoDormant`)))))

(event `GoDormant`
  ;[1 1 1] Update Scale at spawn
  (goto _label :!via `Stop`))

(event `ReverseGrowth`
  ;[1 1 1] Update Scale at spawn
  (if (`self.IsFullyGrown?`)
    (goto _label :!via `ReverseFromEnd`)
    (else
      (goto _label :!via `Reverse`))))

(event `/Game/GAME_FOLDER/CORE/UTILITY/InterfaceEnumsStructs/BPI_Main_Interface.To_Enemy`
  (params (Damage :type "Float (single-precision)") (Hit_Impact_Point :type "Vector Structure") (Hit_Normal :type "Vector Structure") (CritChance :type "Float (single-precision)") (NewParam1 :type "Float (single-precision)"))
  (`/Game/GAME_FOLDER/CORE/BLUEPRINTS/ENEMIES/EnemyHandlerComponent.Hit` (`self.EnemyHandlerComponent`) "NewEnumerator0" (`KismetMathLibrary.RandomFloatInRange` 70.0 300.0) true Hit_Impact_Point))

(fn `Fire`
  ;[1 0.01528 0] fIRE
)

(fn `GetDamage`
  (returns (Damage :type "Float (double-precision)"))
  (return (`.Damage_4_1B70D63441B7CC141681A88AECA237ED` (break `/Game/GAME_FOLDER/CORE/UTILITY/InterfaceEnumsStructs/S_EnemyPodData` (`self.EnemyPodData`)))))

(fn `GetFireRangeRadius`
  (returns (FireRangeRadius :type "Float (double-precision)"))
  (return (`.FireRangeRadius_2_723780534F523D52285445A740F25753` (break `/Game/GAME_FOLDER/CORE/UTILITY/InterfaceEnumsStructs/S_EnemyPodData` (`self.EnemyPodData`)))))

(fn `GetPlayerControllerReference`
  (returns (VaccinController_ref :type "/Game/GAME_FOLDER/CORE/CHARACTER/BP_VaccinController Object Reference"))
  (return null))

(fn `Info_To_UI`
  (returns (Speed_level :type Integer) (Resistance_Level :type Integer) (Dmg_level :type Integer) (Curretn_Resistance :type Integer) (CurrentBodyHealth :type "Float (double-precision)") (AgeInminutes :type Integer))
  (return 0 0 0 0 0.0 0))

(fn `SetFireRangeRadius`
  (`SphereComponent.SetSphereRadius` (`self.FireRange`) (`self.GetFireRangeRadius`) true))

(fn `UserConstructionScript`
  (`parent.UserConstructionScript`)
  (`self.SetFireRangeRadius`))