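; BP_AcidFloor is an acid floor hazard that repeatedly signals damage while the player pawn stands in its DamageArea.
; Overlap starts a looping timer at DamageInterval, and leaving clears it.
; Each tick sends an enum message to the player controller through ToVaccinControllerMessage; an ApplyDamage node using DamageAmount is left unconnected.
; An acid burn sound spawns at the area's location on BeginPlay.
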(event `self.ReceiveBeginPlay`
  ;[1 1 1] Start looping attenuated audio.
  (`GameplayStatics.SpawnSoundAtLocation` "/Game/ASSETS/AUDIO/SFX/Cue_SFX_AcidBurn.Cue_SFX_AcidBurn" (`SceneComponent.K2_GetComponentLocation` (`self.DamageArea`)) (struct) 1.0 1.0 0.0 null null))

(event `self.DamageArea.OnComponentBeginOverlap`
  (params (OverlappedComponent :type "PrimitiveComponent Object Reference") (OtherActor :type "Actor Object Reference") (OtherComp :type "PrimitiveComponent Object Reference") (OtherBodyIndex :type Integer) (bFromSweep :type Boolean) (SweepResult :type "HitResult Structure (by ref)"))
  ;[1 1 1] Start Timer when pawn overlaps.
  (if (== OtherActor (`GameplayStatics.GetPlayerPawn` 0))
    (bind _returnvalue (`KismetSystemLibrary.K2_SetTimerDelegate` (delegate `StartDamage`) (`self.DamageInterval`) true))
    (set `self.DamageTimer` _returnvalue)))

(event `StartDamage`
  (bind _returnvalue (`GameplayStatics.GetPlayerController` 0))
  ;[1 1 1] Continously deals damage if pawn remains in area.
  (`/Engine/EditorBlueprintResources/StandardMacros.IsValid` _returnvalue
    (:`Is Valid`
      (message `/Game/GAME_FOLDER/CORE/UTILITY/InterfaceEnumsStructs/BPI_Main_Interface.To_VaccinController` _returnvalue "NewEnumerator0"))))

(event `self.DamageArea.OnComponentEndOverlap`
  (params (OverlappedComponent :type "PrimitiveComponent Object Reference") (OtherActor :type "Actor Object Reference") (OtherComp :type "PrimitiveComponent Object Reference") (OtherBodyIndex :type Integer))
  ;[1 1 1] Stops timer when pawn exits.
  (if (== OtherActor (`GameplayStatics.GetPlayerPawn` 0))
    (`KismetSystemLibrary.K2_ClearAndInvalidateTimerHandle` (`self.DamageTimer`))))

(fn `UserConstructionScript`)