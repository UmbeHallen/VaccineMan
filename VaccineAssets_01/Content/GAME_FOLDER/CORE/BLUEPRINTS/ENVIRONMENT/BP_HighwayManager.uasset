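; Highway manager that spawns infestation enemy pods on surrounding walls and later removes them.
; SpawnActors sphere-traces randomly within an upward cone from its Arrow, placing tracked pods along hit normals on wall-interface actors, skipping enemies.
; A DoOnce reset by timer rate-limits spawning.
; RemoveSpawnedActors reverses pod growth before a delayed destroy, but the Delay sits inside the loop, so only one pod per call reaches destruction.
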(event `ResetSpawner`
  (bind _returnvalue (`SceneComponent.K2_GetComponentLocation` (`self.Arrow`)))
  (`KismetSystemLibrary.K2_ClearAndInvalidateTimerHandle` (stale `/Game/GAME_FOLDER/CORE/UTILITY/BPInterface_HighwayManager.SpawnActors` _returnvalue_4))
  (goto _label :!via `Reset`))

(event `/Game/GAME_FOLDER/CORE/UTILITY/BPInterface_HighwayManager.SpawnActors`
  (bind _returnvalue (`SceneComponent.K2_GetComponentLocation` (`self.Arrow`)))
  ;[1 1 1] Spawn Infestation Pods randomly in a upwards cone from origin point
  (`/Engine/EditorBlueprintResources/StandardMacros.DoOnce` false :!label _label
    (:`Completed`
      (for _ (range (+ (`self.TraceAmount`) 1))
        (bind (_outhit _returnvalue_2) (`KismetSystemLibrary.SphereTraceSingle` _returnvalue (+ _returnvalue (* (`KismetMathLibrary.RandomUnitVectorInConeInRadians` (`SceneComponent.GetUpVector` (`self.Arrow`)) (`self.ConeHalfAngleInRadians`)) (`self.TraceLength`))) 750.0 "TraceTypeQuery1"))
        (bind (_bblockinghit _binitialoverlap _time _distance _location _impactpoint _normal _impactnormal _physmat _hitactor) (`GameplayStatics.BreakHitResult` _outhit))
        (if (and _returnvalue_2 (`KismetSystemLibrary.DoesImplementInterface` _hitactor "/Game/GAME_FOLDER/CORE/UTILITY/BPInterface_Walls.BPInterface_Walls_C") (not (`KismetSystemLibrary.DoesImplementInterface` _hitactor "/Game/GAME_FOLDER/CORE/UTILITY/InterfaceEnumsStructs/BPI_Enemy_Interface.BPI_Enemy_Interface_C")))
          (bind (_returnvalue_roll _returnvalue_pitch _returnvalue_yaw) (`KismetMathLibrary.BreakRotator` (`KismetMathLibrary.MakeRotFromX` _impactnormal)))
          (bind _returnvalue_3 (`|SpawnActorFromClass` "/Game/GAME_FOLDER/CORE/BLUEPRINTS/ENEMIES/PODS/BASE_POD/BP_MainEnemy_Pod.BP_MainEnemy_Pod_C" (`KismetMathLibrary.MakeTransform` _impactpoint (`KismetMathLibrary.MakeRotator` _returnvalue_roll _returnvalue_pitch _returnvalue_yaw)) "AdjustIfPossibleButAlwaysSpawn" "OverrideRootScale" null null))
          (`KismetArrayLibrary.Array_Add` (`self.SpawnedActors`) _returnvalue_3)))
      (bind _returnvalue_4 (`KismetSystemLibrary.K2_SetTimerDelegate` (delegate `ResetSpawner`) 1.5)))))

(event `/Game/GAME_FOLDER/CORE/UTILITY/BPInterface_HighwayManager.RemoveSpawnedActors`
  ;[1 1 1] Destroys all remaining Spawned Actors.
  (for _array_element (`self.SpawnedActors`)
    (`/Engine/EditorBlueprintResources/StandardMacros.IsValid` _array_element
      (:`Is Valid`
        (`/Game/GAME_FOLDER/CORE/BLUEPRINTS/ENEMIES/PODS/BASE_POD/BP_MainEnemy_Pod.ReverseGrowth` _array_element)
        (`KismetSystemLibrary.Delay` 4.0)
        (`self.K2_DestroyActor` _array_element)))))

(fn `UserConstructionScript`)