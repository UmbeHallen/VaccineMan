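; Area trigger actor that shows a styled primary HUD notification reading "BRAIN" when the first player pawn leaves its Handler volume.
; Forward and rear boxes print a debug string and record entry tags in a unique Direction array when the player overlaps them.
; The switch on the first recorded direction is disconnected, so the notification fires regardless of direction.
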(event `self.ForwardBox.OnComponentBeginOverlap`
  (params (OverlappedComponent :type "PrimitiveComponent Object Reference") (OtherActor :type "Actor Object Reference") (OtherComp :type "PrimitiveComponent Object Reference") (OtherBodyIndex :type Integer) (bFromSweep :type Boolean) (SweepResult :type "HitResult Structure (by ref)"))
  (if (== OtherActor (`GameplayStatics.GetPlayerPawn` 0))
    (`KismetSystemLibrary.PrintString` "FORWARD")
    (`KismetArrayLibrary.Array_AddUnique` (`self.Direction`) "F")))

(event `self.RearBox.OnComponentBeginOverlap`
  (params (OverlappedComponent :type "PrimitiveComponent Object Reference") (OtherActor :type "Actor Object Reference") (OtherComp :type "PrimitiveComponent Object Reference") (OtherBodyIndex :type Integer) (bFromSweep :type Boolean) (SweepResult :type "HitResult Structure (by ref)"))
  (if (== OtherActor (`GameplayStatics.GetPlayerPawn` 0))
    (`KismetSystemLibrary.PrintString` "REAR")
    (`KismetArrayLibrary.Array_AddUnique` (`self.Direction`) "R")))

(event `self.Handler.OnComponentEndOverlap`
  (params (OverlappedComponent :type "PrimitiveComponent Object Reference") (OtherActor :type "Actor Object Reference") (OtherComp :type "PrimitiveComponent Object Reference") (OtherBodyIndex :type Integer))
  (if (== OtherActor (`GameplayStatics.GetPlayerPawn` 0))
    (`/Game/ASSETS/UI/ProHUDV2/Blueprints/Libraries/BPi_HUDManagerV2.CreatePrimaryNotification` (`/Game/ASSETS/UI/ProHUDV2/Blueprints/Libraries/BP_PHV2_Functions.GetHUDManager`) (make `/Game/ASSETS/UI/ProHUDV2/Blueprints/Structs/S_PrimaryNotiInfo` "BRAIN" (make `/Game/ASSETS/UI/ProHUDV2/Blueprints/Structs/S_TextInfo` true (make `SlateFontInfo` "/Game/ASSETS/UI/ProHUDV2/DemoContent/Fonts/BarlowCondensed/F_Barlow_Condensed.F_Barlow_Condensed" "/Engine/VREditor/Fonts/VRTextMaterial.VRTextMaterial") 1.0 (struct :`R` 0.614583 :`B` 0.18523 :`A` 1.0)) "" (struct :`FontInfo` (struct :`OutlineSettings` (struct :`OutlineColor` (struct :`A` 1.0)) :`Size` 24) :`Scale` 1.0 :`ColorAndOpacity` (struct)) (make `/Game/ASSETS/UI/ProHUDV2/Blueprints/Structs/S_IconInfo2` null (struct :`Translation` (0.0 0.0) :`Scale` (1.0 1.0) :`Shear` (0.0 0.0)) (struct :`R` 0.505208 :`G` 0.041623 :`B` 0.061731)) (struct :`R` 0.572385 :`B` 0.614583 :`A` 0.945) 2.0))))

(fn `UserConstructionScript`)