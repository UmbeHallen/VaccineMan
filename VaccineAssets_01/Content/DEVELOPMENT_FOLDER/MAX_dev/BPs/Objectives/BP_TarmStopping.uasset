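; BP_TarmStopping is a breakable cave cliff objective that gives way to a waterfall after repeated hits.
; Each ToEnemy call counts a hit and briefly flashes the cliff white.
; Once the count passes six, after the flash, a timeline scales the waterfall up from zero and the cliff component is destroyed.
; Info_To_UI and GetPlayerControllerReference are stubs returning empty or zero values.
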(event `/Game/GAME_FOLDER/CORE/UTILITY/InterfaceEnumsStructs/BPI_Main_Interface.To_Enemy`
  (params (Damage :type "Float (single-precision)") (Hit_Impact_Point :type "Vector Structure") (Hit_Normal :type "Vector Structure"))
  (bind _sm_cave_cliff_h (`self.SM_cave_cliff_h`))
  (set `self.HitCount` (+ (`self.HitCount`) 1))
  (`PrimitiveComponent.SetMaterial` _sm_cave_cliff_h 0 "/Game/Portals_VFXPack/Materials/M_white.M_white")
  (`KismetSystemLibrary.Delay` 0.1)
  (`PrimitiveComponent.SetMaterial` _sm_cave_cliff_h 0 "/Game/ASSETS/forest_cave/Materials/cave_materials/MI_cave_cliff_g_Inst1.MI_cave_cliff_g_Inst1")
  (if (> (`self.HitCount`) 6)
    (`|ExecutionSequence`
      (:`then_0`
        (bind (_direction _newtrack_0) (`Timeline|Grow`)
          (:`Update`
            (`SceneComponent.SetWorldScale3D` (`self.SM_Waterfall_01`) (`KismetMathLibrary.VLerp` (0.0 0.0 0.0) (5.155 1.695 1.535) _newtrack_0)))))
      (:`then_1`
        (`ActorComponent.K2_DestroyComponent` (`self.SM_cave_cliff_h`))))))

(fn `GetPlayerControllerReference`
  (returns (VaccinController_ref :type "/Game/GAME_FOLDER/CORE/CHARACTER/BP_VaccinController Object Reference"))
  (return null))

(fn `Info_To_UI`
  (returns (Speed_level :type Integer) (Resistance_Level :type Integer) (Dmg_level :type Integer) (Curretn_Resistance :type Integer) (CurrentBodyHealth :type "Float (double-precision)"))
  (return 0 0 0 0 0.0))

(fn `UserConstructionScript`)