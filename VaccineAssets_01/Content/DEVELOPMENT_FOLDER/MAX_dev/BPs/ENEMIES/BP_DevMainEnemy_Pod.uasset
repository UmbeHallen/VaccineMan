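; Stationary-style enemy pod that aims and fires at the player while they are inside its FireRange sphere, sized from EnemyPodData at construction.
; Overlap events toggle the target and a looping Shoot timer that spawns projectiles from an Arrow, while Tick rotates the aim base toward the player.
; ToEnemy reduces health and drives water-bubble hit effects through Niagara and a timeline-animated dynamic material.
; An older slime-shield effect remains unconnected.
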(event `self.ReceiveBeginPlay`
  ;[0 0 0] EVENT TICK
  (`self.DecreaseHealth` -10.0))

(event `self.ReceiveTick`
  (params (DeltaSeconds :type "Float (single-precision)"))
  ;[0 0 0] EVENT TICK
  (`self.LookAtUpdate`))

(event `self.FireRange.OnComponentBeginOverlap`
  (params (OverlappedComponent :type "PrimitiveComponent Object Reference") (OtherActor :type "Actor Object Reference") (OtherComp :type "PrimitiveComponent Object Reference") (OtherBodyIndex :type Integer) (bFromSweep :type Boolean) (SweepResult :type "HitResult Structure (by ref)"))
  (bind _returnvalue (`GameplayStatics.GetPlayerPawn` 0))
  ;[1 0.1 0.1] Detect target unity and save reference variable
  (if (== OtherActor _returnvalue)
    (set `self.Target ref` _returnvalue)
    (set `self.HasTarget` true)
    ;[1 0.1 0.1] Shoot handler and Fire Rate
    (bind _returnvalue_2 (`KismetSystemLibrary.K2_SetTimerDelegate` (delegate `Shoot`) 0.4 true))
    (if (`self.HasTarget`)
      (set `self.FireEventHandler` _returnvalue_2)
      (else
        (`KismetSystemLibrary.K2_ClearAndInvalidateTimerHandle` (`self.FireEventHandler`))))))

(event `Shoot`
  (bind (_returnvalue_location _returnvalue_rotation) (`KismetMathLibrary.BreakTransform` (`SceneComponent.K2_GetComponentToWorld` (`self.Arrow`))))
  ;[1 0.1 0.1] Shoot handler and Fire Rate
  ;[1 0.1 0.1] Shoot Action
  (`|SpawnActorFromClass` "/Game/GAME_FOLDER/CORE/BLUEPRINTS/PROJECTILES/BP_EnemyProjectileBase.BP_EnemyProjectileBase_C" (`KismetMathLibrary.MakeTransform` _returnvalue_location _returnvalue_rotation (3.0 3.0 3.0)) "Undefined" "OverrideRootScale" null null))

(event `self.FireRange.OnComponentEndOverlap`
  (params (OverlappedComponent :type "PrimitiveComponent Object Reference") (OtherActor :type "Actor Object Reference") (OtherComp :type "PrimitiveComponent Object Reference") (OtherBodyIndex :type Integer))
  (bind _returnvalue (`GameplayStatics.GetPlayerPawn` 0))
  ;[1 0.1 0.1] Clear or set new target
  (if (== OtherActor _returnvalue)
    (set `self.HasTarget` false)
    (set `self.Target ref` _returnvalue)
    ;[1 0.1 0.1] Clear shoot timer
    (`KismetSystemLibrary.K2_ClearAndInvalidateTimerHandle` (`self.FireEventHandler`))))

(event `LookAtUpdate`
  (bind (_returnvalue_roll _returnvalue_pitch _returnvalue_yaw) (`KismetMathLibrary.BreakRotator` (`KismetMathLibrary.FindLookAtRotation` (`SceneComponent.K2_GetComponentLocation` (`self.AimBaseComponent`)) (`SceneComponent.K2_GetComponentLocation` (`Actor.RootComponent` (`self.Target ref`))))))
  ;[0 0 0] Look at target
  (if (`self.HasTarget`)
    (`SceneComponent.K2_SetWorldRotation` (`self.AimBaseComponent`) (`KismetMathLibrary.MakeRotator` 0.0 _returnvalue_pitch _returnvalue_yaw) false false)))

(event `/Game/GAME_FOLDER/CORE/UTILITY/InterfaceEnumsStructs/BPI_Main_Interface.To_Enemy`
  (params (Damage :type "Float (single-precision)") (Hit_Impact_Point :type "Vector Structure") (Hit_Normal :type "Vector Structure"))
  (bind _watermat (`self.WaterMat`))
  (`self.DecreaseHealth` Damage)
  (`|ExecutionSequence`
    (:`then_0`
      ;[1 1 1] Niagara
      (`NiagaraComponent.SetVariableVec3` (`self.NPS_WaterBubble`) "Hit_SphereLocation" Hit_Impact_Point)
      ;[1 1 1] Mesh
      (bind _returnvalue (`PrimitiveComponent.CreateDynamicMaterialInstance` (`self.SM_WaterBubble`) 0 "/Game/ASSETS/VFX/Shield_FX_Niagara/Niagara_Shield/Material/M_waterDrop.M_waterDrop" "None"))
      (set `self.WaterMat` _returnvalue)
      (`MaterialInstanceDynamic.SetVectorParameterValue` _returnvalue "Hit_Location" (`KismetMathLibrary.Conv_VectorToLinearColor` Hit_Impact_Point))
      (`NiagaraFunctionLibrary.SpawnSystemAtLocation` "/Game/ASSETS/VFX/Shield_FX_Niagara/Hit_Particles/NS_Hit_Bubble_maxVersion.NS_Hit_Bubble_maxVersion" Hit_Impact_Point (`KismetMathLibrary.MakeRotFromZ` Hit_Normal) (3.0 3.0 3.0))
      (bind (_direction _vertexnoise_strength _hit_opacity _radius_hit _vertexnoise_radius _niagara_hit_radius) (`Timeline|Timeline_1` :!via `PlayFromStart`)
        (:`Update`
          (`NiagaraComponent.SetVariableFloat` (`self.NPS_WaterBubble`) "Hit_SphereRadius" (* _niagara_hit_radius (`self.Niagara_Hit_Radius`)))
          (`MaterialInstanceDynamic.SetScalarParameterValue` _watermat "Radius_VertexNoise" (* _vertexnoise_radius (`self.Radius_VertexNoise`)))
          (`MaterialInstanceDynamic.SetScalarParameterValue` _watermat "Strength_VertexNoise" (* _vertexnoise_strength (`self.VertexNoise_Strength`)))
          (`MaterialInstanceDynamic.SetScalarParameterValue` _watermat "Hit_opacity" _hit_opacity)
          (`MaterialInstanceDynamic.SetScalarParameterValue` _watermat "radius_Hit" (* _radius_hit (`self.radius_Hit`) 0.0)))))))

(fn `Fire`
  ;[1 0.01528 0] fIRE
)

(fn `GetDamage`
  (returns (Damage :type "Float (double-precision)"))
  (return (`.Damage_4_1B70D63441B7CC141681A88AECA237ED` (break `/Game/GAME_FOLDER/CORE/UTILITY/InterfaceEnumsStructs/S_EnemyPodData` (`self.EnemyPodData`)))))

(fn `GetFireRangeRadius`
  (returns (FireRangeRadius :type "Float (double-precision)"))
  (return (`.FireRangeRadius_2_723780534F523D52285445A740F25753` (break `/Game/GAME_FOLDER/CORE/UTILITY/InterfaceEnumsStructs/S_EnemyPodData` (`self.EnemyPodData`)))))

(fn `GetPlayerControllerReference`
  (returns (VaccinController_ref :type "/Game/GAME_FOLDER/CORE/CHARACTER/BP_VaccinController Object Reference"))
  (return null))

(fn `Info_To_UI`
  (returns (Speed_level :type Integer) (Resistance_Level :type Integer) (Dmg_level :type Integer) (Curretn_Resistance :type Integer))
  (return 0 0 0 0))

(fn `SetFireRangeRadius`
  (`SphereComponent.SetSphereRadius` (`self.FireRange`) (`self.GetFireRangeRadius`) true))

(fn `UserConstructionScript`
  (`parent.UserConstructionScript`)
  (`self.SetFireRangeRadius`))