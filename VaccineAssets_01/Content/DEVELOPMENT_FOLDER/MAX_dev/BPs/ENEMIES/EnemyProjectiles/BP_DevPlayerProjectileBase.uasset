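; Base player projectile Blueprint, from a development folder, that deals damage to enemies on hit.
; On Hit, actors implementing BPI_Enemy_Interface receive ToEnemyMessage with a fixed damage value, impact point and normal, avoiding casts to enemy classes.
; The projectile component's bounce event destroys the actor.
; Impact VFX and sound nodes are present but unconnected, and the controller and UI info functions return only empty or zero defaults.
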(event `self.ReceiveHit`
  (params (MyComp :type "PrimitiveComponent Object Reference") (Other :type "Actor Object Reference") (OtherComp :type "PrimitiveComponent Object Reference") (bSelfMoved :type Boolean) (HitLocation :type "Vector Structure") (HitNormal :type "Vector Structure") (NormalImpulse :type "Vector Structure") (Hit :type "HitResult Structure (by ref)"))
  ;[0 0 0] On hit Check
  (if (`KismetSystemLibrary.DoesImplementInterface` Other "/Game/GAME_FOLDER/CORE/UTILITY/InterfaceEnumsStructs/BPI_Enemy_Interface.BPI_Enemy_Interface_C")
    (message `/Game/GAME_FOLDER/CORE/UTILITY/InterfaceEnumsStructs/BPI_Main_Interface.To_Enemy` Other 1.0 Hit_ImpactPoint Hit_ImpactNormal)))

(event `self.Projectile.OnProjectileBounce`
  (params (ImpactResult :type "HitResult Structure (by ref)") (ImpactVelocity :type "Vector Structure (by ref)"))
  (`self.K2_DestroyActor`) ; Then destroy this projectile
)

(fn `GetPlayerControllerReference`
  (returns (VaccinController_ref :type "/Game/GAME_FOLDER/CORE/CHARACTER/BP_VaccinController Object Reference"))
  (return null))

(fn `Info_To_UI`
  (returns (Speed_level :type Integer) (Resistance_Level :type Integer) (Dmg_level :type Integer) (Curretn_Resistance :type Integer))
  (return 0 0 0 0))

(fn `UserConstructionScript`)