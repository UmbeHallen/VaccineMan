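; Base enemy Blueprint that stores health and defense in an EnemyData struct and destroys itself when health runs out.
; Getters expose current and maximum values, and the decrease functions rebuild the struct with the reduced, unclamped stat.
; DecreaseHealth subtracts the damage again from the updated health for its death check, so death can trigger one hit early.
; OnDestroy destroys the actor after a short delay.
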(event `self.OnDestroy`
  ;[1 1 1] On Destort Actor
  (`KismetSystemLibrary.Delay` 0.2)
  (`self.K2_DestroyActor`))

(fn `DecreaseDefense`
  (params (Defense :type "Float (double-precision)"))
  (bind (_icon _name _health _maxhealth _defense _maxdefense) (break `/Game/GAME_FOLDER/CORE/UTILITY/InterfaceEnumsStructs/S_EnemyData` (`self.EnemyData`)))
  (set `self.EnemyData` (make `/Game/GAME_FOLDER/CORE/UTILITY/InterfaceEnumsStructs/S_EnemyData` _icon _name _health _maxhealth (- _defense Defense) _maxdefense)))

(fn `DecreaseHealth`
  (params (Health :type "Float (double-precision)"))
  (bind (_icon _name _health _maxhealth _defense _maxdefense) (break `/Game/GAME_FOLDER/CORE/UTILITY/InterfaceEnumsStructs/S_EnemyData` (`self.EnemyData`)))
  (bind _returnvalue (- _health Health))
  (set `self.EnemyData` (make `/Game/GAME_FOLDER/CORE/UTILITY/InterfaceEnumsStructs/S_EnemyData` _icon _name _returnvalue _maxhealth _defense _maxdefense))
  (if (<= _returnvalue 0.0)
    (`self.OnDestroy`)))

(fn `GetDefense`
  (returns (Defense :type "Float (double-precision)") (`Max Defense` :type "Float (double-precision)"))
  (bind (_icon _name _health _maxhealth _defense _maxdefense) (break `/Game/GAME_FOLDER/CORE/UTILITY/InterfaceEnumsStructs/S_EnemyData` (`self.EnemyData`)))
  (return _defense _maxdefense))

(fn `GetHealth`
  (returns (Health :type "Float (double-precision)") (`Max Health` :type "Float (double-precision)"))
  (bind (_icon _name _health _maxhealth) (break `/Game/GAME_FOLDER/CORE/UTILITY/InterfaceEnumsStructs/S_EnemyData` (`self.EnemyData`)))
  (return _health _maxhealth))

(fn `UserConstructionScript`)