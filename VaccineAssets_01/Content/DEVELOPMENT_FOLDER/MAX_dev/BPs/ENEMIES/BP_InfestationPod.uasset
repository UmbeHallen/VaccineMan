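; BP_InfestationPod is an enemy infestation pod that picks a random type on construction and tints its glass core to suit.
; A random integer roll gives weighted odds for types A, PA, P and E, though a roll of 10 has no case.
; Aggressive type A gets fixed red-orange colours on a dynamic material, while the others get a random blend of two picker colours.
; BeginPlay's type switch and OnHit are empty stubs.
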(event `self.ReceiveBeginPlay`
  (switch `string` (`self.PodType_ID`)))

(event `OnHit`)

(fn `UserConstructionScript`
  ;[0 0 0] MaterialInstance SetUp
  (bind _returnvalue (`PrimitiveComponent.CreateDynamicMaterialInstance` (`self.Core`) 0 "/Game/ASSETS/MATERIALS/MaterialFunctionCollection/Materials/Materials/Edge_Fade/M_StatueGlass_EdgeFade_02_Inst.M_StatueGlass_EdgeFade_02_Inst" "None"))
  (set `self.Core_Material` _returnvalue)
  ;[0 0 0] Randomize TYPE
  (bind _output_get (set `self.PodType_Nr` (`KismetMathLibrary.RandomIntegerInRange` 0 10)))
  (switch `int` _output_get
    (:`0`
      (set `self.PodType_ID` "A" :!label _label))
    (:`1`
      (goto _label))
    (:`2`
      (goto _label))
    (:`3`
      (set `self.PodType_ID` "PA" :!label _label_2))
    (:`4`
      (goto _label_2))
    (:`5`
      (goto _label_2))
    (:`6`
      (goto _label_2))
    (:`7`
      (set `self.PodType_ID` "P" :!label _label_3))
    (:`8`
      (goto _label_3))
    (:`9`
      (set `self.PodType_ID` "E")))
  ;[0 0 0] SET UP ACCORDING TO TYPE
  (switch `string` (`self.PodType_ID`)
    (:`A`
      (`|ExecutionSequence`
        (:`then_0`
          ;[0 0 0] AGGRESIVE TYPE MATERIAL COLOR
          (`MaterialInstanceDynamic.SetVectorParameterValue` (`self.Core_Material`) "ColorGlass" (struct :`R` 1.0 :`G` 0.007345 :`A` 1.0)))
        (:`then_1`
          (`MaterialInstanceDynamic.SetVectorParameterValue` (`self.Core_Material`) "F_Color" (struct :`R` 20.0 :`G` 1.059936 :`A` 1.0)))))
    (:`PA`
      ;[0 0 0] AGGRESIVE TYPE MATERIAL COLOR
      (`MaterialInstanceDynamic.SetVectorParameterValue` (`self.Core_Material`) "ColorGlass" (`KismetMathLibrary.LinearColorLerp` (`self.Color_Picker_A`) (`self.Color_Picker_B`) (`KismetMathLibrary.RandomFloatInRange` 0.0 1.0)) :!label _label_4))
    (:`P`
      (goto _label_4))
    (:`E`
      (goto _label_4))))