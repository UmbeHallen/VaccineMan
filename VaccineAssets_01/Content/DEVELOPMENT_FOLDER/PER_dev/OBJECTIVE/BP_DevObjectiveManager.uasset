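; Development base objective manager that triggers an objective when the first player overlaps its box and the start flag, false at BeginPlay, is set.
; StartObjective and ObjectiveCompleted are empty hooks, with the start logic left to child Blueprints.
; Progress changes are stored only while IsPaused is true, and ObjectiveGeneralCall reports them as severity alongside the objective type.
; It caches a player controller reference, while InfoToUI returns only zeros.
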(event `self.Box.OnComponentBeginOverlap`
  (params (OverlappedComponent :type "PrimitiveComponent Object Reference") (OtherActor :type "Actor Object Reference") (OtherComp :type "PrimitiveComponent Object Reference") (OtherBodyIndex :type Integer) (bFromSweep :type Boolean) (SweepResult :type "HitResult Structure (by ref)"))
  (if (== OtherActor (`GameplayStatics.GetPlayerPawn` 0))
    (if (`self.CanEventStart?`)
      (`self.StartObjective` (`self.Start Delay`)))))

(event `self.ReceiveBeginPlay`
  (bind _vaccincontroller_ref (message `/Game/GAME_FOLDER/CORE/UTILITY/InterfaceEnumsStructs/BPI_Main_Interface.GetPlayerControllerReference` (`GameplayStatics.GetPlayerController` 0)))
  (set `self.Vaccin Controller Ref` _vaccincontroller_ref)
  ;[1 1 1] Conditions for when an event can be activated
  (set `self.CanEventStart?` false))

(event `ChangeProgress`
  (params (`Progress %` :type "Float (double-precision)"))
  (if (`self.Is Paused?`)
    (set `self.ProgressBarPercentage` `Progress %`)))

(event `PauseProgress`
  (params (`IsPaused?` :type Boolean))
  (set `self.Is Paused?` `IsPaused?`))

(event `ObjectiveCompleted`
  ;[1 1 1] HUD Values restored
)

(event `StartObjective`
  (params (StartDelay :type "Float (double-precision)"))
  ;[1 1 1] Save for child.
)

(fn `GetPlayerControllerReference`
  (returns (VaccinController_ref :type "/Game/GAME_FOLDER/CORE/CHARACTER/BP_VaccinController Object Reference"))
  (return null))

(fn `Info_To_UI`
  (returns (Speed_level :type Integer) (Resistance_Level :type Integer) (Dmg_level :type Integer) (Curretn_Resistance :type Integer) (CurrentBodyHealth :type "Float (double-precision)") (AgeInminutes :type Integer))
  (return 0 0 0 0 0.0 0))

(fn `ObjectiveGeneralCall`
  (returns (ObjectiveType :type "/Game/GAME_FOLDER/CORE/UTILITY/InterfaceEnumsStructs/E_ObjectiveType Enum") (ObjectiveSeverity :type "Float (double-precision)"))
  (return (`self.Objective Type`) (`self.ProgressBarPercentage`)))

(fn `UserConstructionScript`)