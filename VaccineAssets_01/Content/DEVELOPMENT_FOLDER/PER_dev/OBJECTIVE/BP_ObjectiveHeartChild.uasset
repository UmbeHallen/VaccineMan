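; Heart objective child Blueprint that hands its objective event to a portal manager in the level.
; On start it pauses progress, finds BP_DevPortalManager, and messages it with the portal count, start delay and a self-reference.
; If no manager exists it only prints a wrong-objective warning.
; HeartEventCompleted marks the objective complete; a leftover progress reset is unconnected.
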(event `self.ReceiveBeginPlay`
  (`parent.ReceiveBeginPlay`))

(event `self.StartObjective`
  (params (StartDelay :type "Float (single-precision)"))
  ;[1 1 1] check if there is a portal manager already
  (`self.PauseProgress` true)
  (bind _returnvalue (`GameplayStatics.GetActorOfClass` "/Game/DEVELOPMENT_FOLDER/PER_dev/HEART_OBJECTIVE/ENEMIES/BP_DevPortalManager.BP_DevPortalManager_C"))
  (`/Engine/EditorBlueprintResources/StandardMacros.IsValid` _returnvalue
    (:`Is Valid`
      (bind _output_get (set `self.PortalManager` _returnvalue))
      (message `/Game/GAME_FOLDER/CORE/UTILITY/BPInterface_Objective.GetAmountOfPortals` _output_get (`self.AmountOfPortals`))
      (message `/Game/GAME_FOLDER/CORE/UTILITY/BPInterface_Objective.StartEvent` (`self.PortalManager`) StartDelay self))
    (:`Is Not Valid`
      (`KismetSystemLibrary.PrintString` "Wrong Objective Selected"))))

(event `/Game/GAME_FOLDER/CORE/UTILITY/BPInterface_Objective.HeartEventCompleted`
  (`self.ObjectiveCompleted`))

(fn `UserConstructionScript`
  (`parent.UserConstructionScript`))