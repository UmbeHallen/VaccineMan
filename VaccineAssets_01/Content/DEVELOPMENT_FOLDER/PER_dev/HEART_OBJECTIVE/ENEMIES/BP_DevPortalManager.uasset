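; Manager for the heart objective event that spawns a timed series of BP_DevPortal actors around itself.
; StartEvent waits, loops SpawnPortal through a delayed-loop macro, then calls HeartEventCompleted on the object manager.
; Each portal spawns facing the manager at a random wide-cone point TraceLength from its arrow; the line trace result is unused.
; Each is told to despawn shortly before the next spawn, based on TimeBetweenPortalsSpawning.
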(event `/Game/GAME_FOLDER/CORE/UTILITY/BPInterface_Objective.StartEvent`
  (params (StartDelay :type "Float (single-precision)") (ObjectManagerRef :type "/Game/DEVELOPMENT_FOLDER/PER_dev/OBJECTIVE/BP_DevObjectiveManager Object Reference"))
  ;[1 1 1] Set initial delay and start spawning event.
  (set `self.Object Manager Ref` ObjectManagerRef)
  (`KismetSystemLibrary.Delay` StartDelay)
  (`self.ForLoopWithDelay` 1 (`self.Amount Of Portals`) (`self.SpawnInterval`)
    (:`ExecOut`
      (`self.SpawnPortal`))
    (:`Completed`
      (`/Game/DEVELOPMENT_FOLDER/PER_dev/OBJECTIVE/BP_DevObjectiveManager.HeartEventCompleted` (`self.Object Manager Ref`)))))

(event `SpawnPortal`
  ;[1 1 1] Line trace to find area to spawn portal.
  (if (`self.SpawnPortals?`)
    (set `self.SpawnLocation` (+ (`SceneComponent.K2_GetComponentLocation` (`self.Arrow`)) (* (`KismetMathLibrary.RandomUnitVectorInConeInRadians` (`SceneComponent.GetUpVector` (`self.Arrow`)) 3.0) (`self.TraceLength`))))
    (`KismetSystemLibrary.LineTraceSingle` (`SceneComponent.K2_GetComponentLocation` (`self.Arrow`)) (`self.SpawnLocation`) "TraceTypeQuery1")
    ;[1 1 1] Spawn a portal that's facing the manager at the trace's end location.
    (bind _returnvalue (`|SpawnActorFromClass` "/Game/DEVELOPMENT_FOLDER/PER_dev/HEART_OBJECTIVE/ENEMIES/BP_DevPortal.BP_DevPortal_C" (`KismetMathLibrary.MakeTransform` (`self.SpawnLocation`) (`KismetMathLibrary.FindLookAtRotation` (`self.SpawnLocation`) (`SceneComponent.K2_GetComponentLocation` (`self.Arrow`)))) "AdjustIfPossibleButAlwaysSpawn" "OverrideRootScale" null null))
    (set `self.SpawnedPortal` _returnvalue)
    (`self.RemoveCurrentPortal`)))

(event `RemoveCurrentPortal`
  ;[1 1 1] Tell current portal to initate removal after a delay.
  (`KismetSystemLibrary.Delay` (- (`self.SpawnInterval`) (`self.TimeBetweenPortalsSpawning`)))
  (`/Game/DEVELOPMENT_FOLDER/PER_dev/HEART_OBJECTIVE/ENEMIES/BP_DevPortal.DespawnPortal` (`self.SpawnedPortal`)))

(event `/Game/GAME_FOLDER/CORE/UTILITY/BPInterface_Objective.GetAmountOfPortals`
  (params (AmountOfPortals :type Integer))
  ;[1 1 1] Get amount of portals from objective manager.
  (set `self.Amount Of Portals` AmountOfPortals))

(fn `UserConstructionScript`)