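; Kamikaze enemy that homes in on the BP_DevNewHeart objective and calls OnDestroy when it arrives.
; On BeginPlay two timelines run together, with play rates set by HoningSpeed and OffsetSpeed.
; One lerps the actor to the heart's initial location, while the other sweeps the mesh toward a relative offset, layering the motions.
; Tick feeds the mesh's world position to Niagara so particles follow it.
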(event `self.ReceiveTick`
  (params (DeltaSeconds :type "Float (single-precision)"))
  ;[1 1 1] Update Particle location.
  (`NiagaraComponent.SetVariableVec3` (`self.Niagara`) "ParPos" (`SceneComponent.K2_GetComponentLocation` (`self.StaticMesh`))))

(event `self.ReceiveBeginPlay`
  ;[1 1 1] Set up target and locations.
  (bind _returnvalue (`GameplayStatics.GetActorOfClass` "/Game/DEVELOPMENT_FOLDER/PER_dev/HEART_OBJECTIVE/BP_DevNewHeart.BP_DevNewHeart_C"))
  (bind _output_get (set `self.Target` _returnvalue))
  (set `self.TargetLocation` (`self.K2_GetActorLocation` _output_get))
  (set `self.StartingLocation` (`self.K2_GetActorLocation`))
  ;[1 1 1] Customize Timeline play rates.
  (`TimelineComponent.SetPlayRate` (`self.HoneInOnHeart`) (/ 1.0 (`self.HoningSpeed`)))
  (`TimelineComponent.SetPlayRate` (`self.GoToOffset`) (/ 1.0 (`self.OffsetSpeed`)))
  (`|ExecutionSequence`
    (:`then_0`
      ;[1 1 1] Move actor from start location to the target.
      (bind (_direction _alpha) (`Timeline|HoneInOnHeart` :!via `PlayFromStart`)
        (:`Update`
          (`self.K2_SetActorLocation` (`KismetMathLibrary.VLerp` (`self.StartingLocation`) (`self.TargetLocation`) _alpha)))
        (:`Finished`
          (`self.OnDestroy`))))
    (:`then_1`
      ;[1 1 1] Move mesh to an offset location from itself.
      (bind (_direction_2 _alpha_2) (`Timeline|GoToOffset`)
        (:`Update`
          (`SceneComponent.K2_SetRelativeLocation` (`self.StaticMesh`) (`KismetMathLibrary.VLerp` (0.0 0.0 0.0) (`self.OffsetLocation`) _alpha_2) true false))
        (:`SetOffsetPoint`
          (set `self.MeshLocationInOffset` (`SceneComponent.K2_GetComponentLocation` (`self.StaticMesh`))))))))

(fn `UserConstructionScript`
  (`parent.UserConstructionScript`))