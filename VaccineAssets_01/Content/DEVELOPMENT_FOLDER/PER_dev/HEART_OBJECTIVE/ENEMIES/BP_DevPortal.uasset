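; BP_DevPortal is a development portal actor that spawns BP_DevKamikazeEnemy instances at a regular interval.
; A looping timer started on BeginPlay spawns each enemy at the Arrow component's transform, adjusting for collisions but always spawning.
; Each enemy then takes the portal's pitch and yaw with a randomized roll.
; A DespawnPortal event destroys the portal.
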(event `self.ReceiveBeginPlay`
  ;[1 1 1] Initiate portal event.
  (`KismetSystemLibrary.K2_SetTimerDelegate` (delegate `SpawnEnemy`) (`self.SpawnInterval`) true))

(event `SpawnEnemy`
  (bind (_returnvalue_roll _returnvalue_pitch _returnvalue_yaw) (`KismetMathLibrary.BreakRotator` (`self.K2_GetActorRotation`)))
  (bind _arrow (`self.Arrow`))
  ;[1 1 1] Spawn Enemies with even intervals and give them random rotations.
  (bind _returnvalue (`|SpawnActorFromClass` "/Game/DEVELOPMENT_FOLDER/PER_dev/HEART_OBJECTIVE/ENEMIES/BP_DevKamikazeEnemy.BP_DevKamikazeEnemy_C" (`KismetMathLibrary.MakeTransform` (`SceneComponent.K2_GetComponentLocation` _arrow) (`SceneComponent.K2_GetComponentRotation` _arrow)) "AdjustIfPossibleButAlwaysSpawn" "OverrideRootScale" null null))
  (bind _returnvalue_roll_2 (`KismetMathLibrary.BreakRotator` (`self.K2_GetActorRotation` _returnvalue)))
  (`self.K2_SetActorRotation` _returnvalue (`KismetMathLibrary.MakeRotator` (+ _returnvalue_roll_2 (`KismetMathLibrary.RandomFloatInRange` 1.0 360.0)) _returnvalue_pitch _returnvalue_yaw) false))

(event `DespawnPortal`
  ;[1 1 1] Remove portal.
  (`self.K2_DestroyActor`))

(fn `UserConstructionScript`)