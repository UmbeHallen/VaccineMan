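; Development version of a heart objective actor with a blood shield sphere that reacts visually to overlaps at the impact point.
; Each overlap sends the hit location to the shield's Niagara system and a new dynamic material instance, and spawns a blood hit effect.
; A timeline then drives Niagara hit radius, vertex noise and hit opacity, though the material's hit radius is multiplied by zero.
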(event `self.ReceiveBeginPlay`
  ;[1 1 1] Enable controller input.
  (`self.EnableInput` (`GameplayStatics.GetPlayerController` 0)))

(event `self.SM_Sphere.OnComponentBeginOverlap`
  (params (OverlappedComponent :type "PrimitiveComponent Object Reference") (OtherActor :type "Actor Object Reference") (OtherComp :type "PrimitiveComponent Object Reference") (OtherBodyIndex :type Integer) (bFromSweep :type Boolean) (SweepResult :type "HitResult Structure (by ref)"))
  (bind (_bblockinghit _binitialoverlap _time _distance _location _impactpoint _normal _impactnormal) (`GameplayStatics.BreakHitResult` SweepResult))
  ;[1 1 1] Set hit location niagara variable.
  (`NiagaraComponent.SetVariableVec3` (`self.NS_Shield_Sphere`) "Hit_SphereLocation" _impactpoint)
  ;[1 1 1] Create material instance.
  (bind _returnvalue (`PrimitiveComponent.CreateDynamicMaterialInstance` (`self.SM_Sphere`) 0 "/Game/ASSETS/VFX/Shield_FX_Niagara/Niagara_Shield/Material/M_Shield_Blood.M_Shield_Blood" "None"))
  (bind _output_get (set `self.MaterialInstance` _returnvalue))
  ;[1 1 1] Mesh
  (`MaterialInstanceDynamic.SetVectorParameterValue` _output_get "Hit_Location" (`KismetMathLibrary.Conv_VectorToLinearColor` _impactpoint))
  (`NiagaraFunctionLibrary.SpawnSystemAtLocation` "/Game/ASSETS/VFX/Shield_FX_Niagara/Hit_Particles/NS_Hit_Blood.NS_Hit_Blood" _impactpoint (`KismetMathLibrary.MakeRotFromZ` _impactnormal))
  (bind (_direction _vertexnoise_strength _hit_opacity _radius_hit _vertexnoise_radius _niagara_hit_radius) (`Timeline|Mesh_Timeline` :!via `PlayFromStart`)
    (:`Update`
      (`NiagaraComponent.SetVariableFloat` (`self.NS_Shield_Sphere`) "Hit_SphereRadius" (* _niagara_hit_radius (`self.Niagara_Hit_Radius`)))
      (`MaterialInstanceDynamic.SetScalarParameterValue` (`self.MaterialInstance`) "Radius_VertexNoise" (* _vertexnoise_radius (`self.Radius_VertexNoise`)))
      (`MaterialInstanceDynamic.SetScalarParameterValue` (`self.MaterialInstance`) "Strength_VertexNoise" (* _vertexnoise_strength (`self.VertexNoise_Strength`)))
      (`MaterialInstanceDynamic.SetScalarParameterValue` (`self.MaterialInstance`) "Hit_opacity" _hit_opacity)
      (`MaterialInstanceDynamic.SetScalarParameterValue` (`self.MaterialInstance`) "radius_Hit" (* _radius_hit (`self.radius_Hit`) 0.0)))))

(fn `UserConstructionScript`)